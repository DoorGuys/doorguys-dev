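; Door variation controller actor that swaps styles and materials across arrays of standard, sliding and barn doors.
; ChangeVarID takes an ID and tag, routing to mesh swaps and tag-matched material variations, applied by part type through each door's PartsForVariations.
; Door and glass meshes change on all three types; frames and hardware only on standard doors, as the sliding frame loop is empty.
; Handle and entry handle tags call each other's swap functions.
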(event `/Game/DoorsBPV2/Blueprints/Others/BPI_Doors_Interaction.Change Var ID`
  (params (ChangeToID :type Integer) (TagIn :type String))
  (`|ExecutionSequence`
    (:`then_0`
      (if (`KismetStringLibrary.EqualEqual_StrStr` TagIn (`self.Tag Door Style`))
        (`self.Swap Door Style` ChangeToID)))
    (:`then_1`
      (if (`KismetStringLibrary.EqualEqual_StrStr` (`self.Tag Frame Style`) TagIn)
        (`self.Swap Frame Style` ChangeToID)))
    (:`then_2`
      (`self.Swap Materials` ChangeToID TagIn))
    (:`then_3`
      (if (`KismetStringLibrary.EqualEqual_StrStr` TagIn (`self.Tag Handle Style`))
        (`self.Swap Entry Handle Style` ChangeToID)))
    (:`then_4`
      (if (`KismetStringLibrary.EqualEqual_StrStr` TagIn (`self.Tag Entry Handle Style`))
        (`self.Swap Handle Style` ChangeToID)))
    (:`then_5`
      (if (`KismetStringLibrary.EqualEqual_StrStr` TagIn (`self.Tag Plate Style`))
        (`self.Swap Plate Style` ChangeToID)))))

(fn `Get Material Array from Var ID`
  (params (`Material Variations` :type "Array of /Game/DoorsBPV2/Blueprints/Structs/BPS_VarMatIds Structure") (ID :type Integer))
  (returns (Materials :type "Array of MaterialInterface Object Reference"))
  (`KismetArrayLibrary.Array_Clear` (`self.Material Array`))
  (for _array_element `Material Variations`
    (bind (_id _materials) (break `/Game/DoorsBPV2/Blueprints/Structs/BPS_VarMatIds` _array_element))
    (`KismetArrayLibrary.Array_Set` (`self.Material Array`) _id (`|GetArrayItem` _materials ID) true))
  (return (`self.Material Array`)))

(fn `Set Material IDs`
  (params (`Var Parts` :type "Array of /Game/DoorsBPV2/Blueprints/Structs/BPS_PartsForVariations Structure") (Material :type "Array of MaterialInterface Object Reference") (`Part Type` :type "/Game/DoorsBPV2/Blueprints/Enums/Enum_DoorVarParts Enum" :default "NewEnumerator23"))
  (for _array_element `Var Parts`
    (bind (_component _part) (break `/Game/DoorsBPV2/Blueprints/Structs/BPS_PartsForVariations` _array_element))
    (if (`|EnumEquality` _part `Part Type`)
      (if (`KismetArrayLibrary.Array_IsValidIndex` Material)
        (for (_array_element_2 _array_index) Material
          (`/Engine/EditorBlueprintResources/StandardMacros.IsValid` _array_element_2
            (:`Is Valid`
              (`PrimitiveComponent.SetMaterial` _component _array_index _array_element_2))))))))

(fn `Swap Door Style`
  (params (`Style ID` :type Integer))
  (bind _output (`|GetArrayItem` (`self.Door Style`) `Style ID`))
  (`|ExecutionSequence`
    (:`then_0`
      ;[1 1 1 0.5] Standard
      (for _array_element (`self.BP_StandardDoors`)
        (bind _partsforvariations (`/Game/DoorsBPV2/Blueprints/BP_StandardDoor.PartsForVariations` _array_element))
        (bind (_door _glass) (`/Game/DoorsBPV2/Blueprints/Others/BPL_UniDoors.Get Door Meshes` (`/Game/DoorsBPV2/Blueprints/BP_StandardDoor.GetSizeType` _array_element) _output))
        (`self.Swap Mesh` _partsforvariations _door "NewEnumerator0") ; Door
        (`self.Swap Mesh` _partsforvariations _glass "NewEnumerator8") ; Glass
      ))
    (:`then_1`
      ;[1 1 1 0.5] Sliding
      (for _array_element_2 (`self.BP_SlidingDoors`)
        (bind _parts_for_variations (`/Game/DoorsBPV2/Blueprints/BP_SlidingDoor.Parts for Variations` _array_element_2))
        (bind (_door_2 _glass_2) (`/Game/DoorsBPV2/Blueprints/Others/BPL_UniDoors.Get Door Meshes` (`/Game/DoorsBPV2/Blueprints/BP_SlidingDoor.GetSizeType` _array_element_2) _output))
        (`self.Swap Mesh` _parts_for_variations _door_2 "NewEnumerator0")
        (`self.Swap Mesh` _parts_for_variations _glass_2 "NewEnumerator8")))
    (:`then_2`
      ;[1 1 1 0.5] Barn
      (for _array_element_3 (`self.BP_BarnDoors`)
        (bind _parts_for_variations_2 (`/Game/DoorsBPV2/Blueprints/BP_BarnDoor.Parts for Variations` _array_element_3))
        (bind (_door_3 _glass_3) (`/Game/DoorsBPV2/Blueprints/Others/BPL_UniDoors.Get Door Meshes` (`/Game/DoorsBPV2/Blueprints/BP_BarnDoor.GetSizeType` _array_element_3) _output))
        (`self.Swap Mesh` _parts_for_variations_2 _door_3 "NewEnumerator0")
        (`self.Swap Mesh` _parts_for_variations_2 _glass_3 "NewEnumerator8")))))

(fn `Swap Entry Handle Style`
  (params (`Variation ID` :type Integer))
  (`self.Swap Hardware Style` "NewEnumerator9" (`/Game/DoorsBPV2/Blueprints/Others/BPL_UniHardware.Get Entry Handle Mesh` (`|GetArrayItem` (`self.Entry Handle Styles (Std)`) `Variation ID`))))

(fn `Swap Frame Style`
  (params (`Style ID` :type Integer))
  (`|ExecutionSequence`
    (:`then_0`
      (for _array_element (`self.BP_StandardDoors`)
        (for _array_element_2 (`/Game/DoorsBPV2/Blueprints/BP_StandardDoor.PartsForVariations` _array_element)
          (bind (_component _part) (break `/Game/DoorsBPV2/Blueprints/Structs/BPS_PartsForVariations` _array_element_2))
          (if (`|EnumEquality` _part "NewEnumerator1")
            (`StaticMeshComponent.SetStaticMesh` _component (`/Game/DoorsBPV2/Blueprints/Others/BPL_UniDoors.Get Frame Mesh` (`|GetArrayItem` (`self.Frame Style`) `Style ID`) (`/Game/DoorsBPV2/Blueprints/BP_StandardDoor.GetSizeType` _array_element) (`/Game/DoorsBPV2/Blueprints/BP_StandardDoor.IsDoubleDoor` _array_element)))))))
    (:`then_1`
      (for _array_element_3 (`self.BP_SlidingDoors`)
        _))))

(fn `Swap Handle Style`
  (params (`Variation ID` :type Integer))
  (`self.Swap Hardware Style` "NewEnumerator4" (`/Game/DoorsBPV2/Blueprints/Others/BPL_UniHardware.Get Handle Mesh` (`|GetArrayItem` (`self.Handle Styles (Std)`) `Variation ID`))))

(fn `Swap Hardware Style`
  (params (`Variation Part` :type "/Game/DoorsBPV2/Blueprints/Enums/Enum_DoorVarParts Enum" :default "NewEnumerator0") (`New Mesh` :type "StaticMesh Object Reference"))
  (for _array_element (`self.BP_StandardDoors`)
    (for _array_element_2 (`/Game/DoorsBPV2/Blueprints/BP_StandardDoor.PartsForVariations` _array_element)
      (bind (_component _part) (break `/Game/DoorsBPV2/Blueprints/Structs/BPS_PartsForVariations` _array_element_2))
      (if (`|EnumEquality` _part `Variation Part`)
        (`StaticMeshComponent.SetStaticMesh` _component `New Mesh`)))))

(fn `Swap Materials`
  (params (`Variation ID` :type Integer) (Tag :type String))
  (for _array_element (`self.Material Variations`)
    (bind (_part _variations _tag) (break `/Game/DoorsBPV2/Blueprints/Structs/BPS_VarMaterials` _array_element))
    (if (`KismetStringLibrary.EqualEqual_StrStr` _tag Tag)
      (for _array_element_2 _part
        (`|ExecutionSequence`
          (:`then_0`
            (for _array_element_3 (`self.BP_StandardDoors`)
              (bind _materials (`self.Get Material Array from Var ID` _variations `Variation ID`))
              (`self.Set Material IDs` (`/Game/DoorsBPV2/Blueprints/BP_StandardDoor.PartsForVariations` _array_element_3) _materials _array_element_2)))
          (:`then_1`
            (for _array_element_4 (`self.BP_SlidingDoors`)
              (`self.Set Material IDs` (`/Game/DoorsBPV2/Blueprints/BP_SlidingDoor.Parts for Variations` _array_element_4) _materials _array_element_2)))
          (:`then_2`
            (for _array_element_5 (`self.BP_BarnDoors`)
              (`self.Set Material IDs` (`/Game/DoorsBPV2/Blueprints/BP_BarnDoor.Parts for Variations` _array_element_5) _materials _array_element_2))))))))

(fn `Swap Mesh`
  (params (`Part Array` :type "Array of /Game/DoorsBPV2/Blueprints/Structs/BPS_PartsForVariations Structure") (`New Mesh` :type "StaticMesh Object Reference") (`Var Part` :type "/Game/DoorsBPV2/Blueprints/Enums/Enum_DoorVarParts Enum" :default "NewEnumerator23"))
  (for _array_element `Part Array`
    (bind (_component _part) (break `/Game/DoorsBPV2/Blueprints/Structs/BPS_PartsForVariations` _array_element))
    (if (`|EnumEquality` _part `Var Part`)
      (`SceneComponent.SetMobility` _component "Movable") ; Set Movable so it can be changed
      (`StaticMeshComponent.SetStaticMesh` _component `New Mesh`) ; Set New Mesh
    )))

(fn `Swap Plate Style`
  (params (`Variation ID` :type Integer))
  (`self.Swap Hardware Style` "NewEnumerator5" (`/Game/DoorsBPV2/Blueprints/Others/BPL_UniHardware.Get Plate Mesh` (`|GetArrayItem` (`self.Plate Styles (Std)`) `Variation ID`))))

(fn `UserConstructionScript`)