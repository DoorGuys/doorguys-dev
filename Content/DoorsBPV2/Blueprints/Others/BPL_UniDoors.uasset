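; Blueprint function library for modular doors that picks meshes and computes sizing and transforms.
; GetDoorDetails maps AU, DIN EN and US sizes to six mesh classes plus width/height scale factors.
; Select-based getters resolve door, glass, frame and top-window meshes by style, class and, for frames, single or double.
; Transform helpers handle mirroring, offsets and frame scaling, and fit custom meshes from their bounds, snapping yaw to quarter turns.
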(fn `Add Offset Z`
  (params (InTransform :type "Transform Structure (by ref)") (Offset :type "Float (double-precision)"))
  (returns (Transform :type "Transform Structure"))
  (return (`KismetMathLibrary.MakeTransform` (`KismetMathLibrary.MakeVector` (.x (.location InTransform)) (.y (.location InTransform)) (+ Offset (.z (.location InTransform)))) (.rotation InTransform) (.scale InTransform))))

(fn `Combine Transforms`
  (params (`Transform 1` :type "Transform Structure (by ref)") (`Transform 2` :type "Transform Structure (by ref)"))
  (returns (Combined :type "Transform Structure"))
  (return (`KismetMathLibrary.MakeTransform` (+ (.location `Transform 1`) (.location `Transform 2`)) (`KismetMathLibrary.ComposeRotators` (.rotation `Transform 1`) (.rotation `Transform 2`)) (* (.scale `Transform 1`) (.scale `Transform 2`)))))

(fn `Get Custom Scale`
  (params (size :type "/Game/DoorsBPV2/Blueprints/Enums/Enum_DoorSizes Enum" :default "NewEnumerator12") (DoorMesh :type "StaticMesh Object Reference") (ThicknessScale :type "Float (double-precision)" :default 1.0) (Transform :type "Transform Structure"))
  (returns (Scale :type "Vector Structure") (Offset :type "Vector Structure"))
  (bind (_origin _boxextent) (`KismetMathLibrary.BreakBoxSphereBounds` (`StaticMesh.GetBounds` DoorMesh)))
  (bind _yaw (.yaw (.rotation Transform)))
  (bind _x (.x _origin))
  (bind _y (.y _origin))
  (bind _x_2 (.x _boxextent))
  (bind _y_2 (.y _boxextent))
  (bind _returnvalue (select `/Game/DoorsBPV2/Blueprints/Enums/Enum_SizeType` (`.Size_31_B8433DE84B64E774499717A1BF6F598E` (break `/Game/DoorsBPV2/Blueprints/Structs/BPS_DoorSizes` (`self.Get Door Details` size))) :`NewEnumerator0` (36.0 4.0 102.0) :`NewEnumerator1` (41.0 4.0 102.0) :`NewEnumerator2` (46.0 4.0 102.0) :`NewEnumerator3` (36.0 4.0 117.0) :`NewEnumerator4` (41.0 4.0 117.0) :`NewEnumerator5` (46.0 4.0 117.0) :!type "Vector Structure"))
  (bind _returnvalue_2 (* _x ThicknessScale))
  (bind _returnvalue_3 (* _y ThicknessScale))
  (bind _returnvalue_4 (/ (.z _returnvalue) (.z _boxextent)))
  (bind _returnvalue_5 (/ (.x _returnvalue) (.x _boxextent)))
  (bind _returnvalue_6 (/ (.x _returnvalue) (.y _boxextent)))
  (bind _returnvalue_7 (`KismetMathLibrary.MakeVector` ThicknessScale _returnvalue_6 _returnvalue_4))
  (bind _returnvalue_8 (`KismetMathLibrary.MakeVector` _returnvalue_5 ThicknessScale (/ (.z _returnvalue) (.z _boxextent))))
  (bind _returnvalue_9 (select `bool` (< _yaw 5.0) :`false` (select `bool` (< _yaw 95.0) :`false` (select `bool` (< _yaw 185.0) :`false` "NewEnumerator3" :`true` "NewEnumerator2" :!type "/Game/DoorsBPV2/Blueprints/Enums/Enum_Rotation Enum") :`true` "NewEnumerator1") :`true` "NewEnumerator0"))
  (bind _returnvalue_10 (* (select `/Game/DoorsBPV2/Blueprints/Enums/Enum_Rotation` _returnvalue_9 :`NewEnumerator0` (- _y _y_2) :`NewEnumerator1` (- _x _x_2) :`NewEnumerator2` (+ _y _y_2) :`NewEnumerator3` (+ _x _x_2)) (select `/Game/DoorsBPV2/Blueprints/Enums/Enum_Rotation` _returnvalue_9 :`NewEnumerator0` _returnvalue_6 :`NewEnumerator1` _returnvalue_5 :`NewEnumerator2` _returnvalue_6 :`NewEnumerator3` _returnvalue_5) -1.0))
  (`|ExecutionSequence`
    (:`then_1`
      (`/Engine/EditorBlueprintResources/StandardMacros.IsValid` DoorMesh
        (:`Is Valid`
          (return (select `/Game/DoorsBPV2/Blueprints/Enums/Enum_Rotation` _returnvalue_9 :`NewEnumerator0` _returnvalue_7 :`NewEnumerator1` _returnvalue_8 :`NewEnumerator2` _returnvalue_7 :`NewEnumerator3` _returnvalue_8) (`KismetMathLibrary.MakeVector` (select `/Game/DoorsBPV2/Blueprints/Enums/Enum_Rotation` _returnvalue_9 :`NewEnumerator0` (- -2.0 _returnvalue_2) :`NewEnumerator1` _returnvalue_10 :`NewEnumerator2` (- 2.0 _returnvalue_2) :`NewEnumerator3` _returnvalue_10) (select `/Game/DoorsBPV2/Blueprints/Enums/Enum_Rotation` _returnvalue_9 :`NewEnumerator0` _returnvalue_10 :`NewEnumerator1` (- 2.0 _returnvalue_3) :`NewEnumerator2` _returnvalue_10 :`NewEnumerator3` (- -2.0 _returnvalue_3)) (* _returnvalue_4 (- (.z _boxextent) (.z _origin))))))))))

(fn `Get Door 04`
  (params (Size :type "/Game/DoorsBPV2/Blueprints/Enums/Enum_SizeType Enum" :default "NewEnumerator0"))
  (returns (`Door Mesh` :type "StaticMesh Object Reference") (`Glass Mesh` :type "StaticMesh Object Reference"))
  (return (select `/Game/DoorsBPV2/Blueprints/Enums/Enum_SizeType` Size :`NewEnumerator0` "/Game/DoorsBPV2/Meshes/Doors/04/SM_S_Door04.SM_S_Door04" :`NewEnumerator1` "/Game/DoorsBPV2/Meshes/Doors/04/SM_M_Door04.SM_M_Door04" :`NewEnumerator2` "/Game/DoorsBPV2/Meshes/Doors/04/SM_L_Door04.SM_L_Door04" :`NewEnumerator3` "/Game/DoorsBPV2/Meshes/Doors/04/SM_SH_Door04.SM_SH_Door04" :`NewEnumerator4` "/Game/DoorsBPV2/Meshes/Doors/04/SM_MH_Door04.SM_MH_Door04" :`NewEnumerator5` "/Game/DoorsBPV2/Meshes/Doors/04/SM_LH_Door04.SM_LH_Door04" :!type "StaticMesh Object Reference") (select `/Game/DoorsBPV2/Blueprints/Enums/Enum_SizeType` Size :`NewEnumerator0` "/Game/DoorsBPV2/Meshes/Doors/04/SM_S_Door04_Glass.SM_S_Door04_Glass" :`NewEnumerator1` "/Game/DoorsBPV2/Meshes/Doors/04/SM_M_Door04_Glass.SM_M_Door04_Glass" :`NewEnumerator2` "/Game/DoorsBPV2/Meshes/Doors/04/SM_L_Door04_Glass.SM_L_Door04_Glass" :`NewEnumerator3` "/Game/DoorsBPV2/Meshes/Doors/04/SM_SH_Door04_Glass.SM_SH_Door04_Glass" :`NewEnumerator4` "/Game/DoorsBPV2/Meshes/Doors/04/SM_MH_Door04_Glass.SM_MH_Door04_Glass" :`NewEnumerator5` "/Game/DoorsBPV2/Meshes/Doors/04/SM_LH_Door04_Glass.SM_LH_Door04_Glass" :!type "StaticMesh Object Reference")))

(fn `Get Door 05`
  (params (Size :type "/Game/DoorsBPV2/Blueprints/Enums/Enum_SizeType Enum" :default "NewEnumerator0"))
  (returns (`Door Mesh` :type "StaticMesh Object Reference") (`Glass Mesh` :type "StaticMesh Object Reference"))
  (return (select `/Game/DoorsBPV2/Blueprints/Enums/Enum_SizeType` Size :`NewEnumerator0` "/Game/DoorsBPV2/Meshes/Doors/05/SM_S_Door05.SM_S_Door05" :`NewEnumerator1` "/Game/DoorsBPV2/Meshes/Doors/05/SM_M_Door05.SM_M_Door05" :`NewEnumerator2` "/Game/DoorsBPV2/Meshes/Doors/05/SM_L_Door05.SM_L_Door05" :`NewEnumerator3` "/Game/DoorsBPV2/Meshes/Doors/05/SM_SH_Door05.SM_SH_Door05" :`NewEnumerator4` "/Game/DoorsBPV2/Meshes/Doors/05/SM_MH_Door05.SM_MH_Door05" :`NewEnumerator5` "/Game/DoorsBPV2/Meshes/Doors/05/SM_LH_Door05.SM_LH_Door05" :!type "StaticMesh Object Reference") (select `/Game/DoorsBPV2/Blueprints/Enums/Enum_SizeType` Size :`NewEnumerator0` "/Game/DoorsBPV2/Meshes/Doors/05/SM_S_Door05_Glass.SM_S_Door05_Glass" :`NewEnumerator1` "/Game/DoorsBPV2/Meshes/Doors/05/SM_M_Door05_Glass.SM_M_Door05_Glass" :`NewEnumerator2` "/Game/DoorsBPV2/Meshes/Doors/05/SM_L_Door05_Glass.SM_L_Door05_Glass" :`NewEnumerator3` "/Game/DoorsBPV2/Meshes/Doors/05/SM_SH_Door05_Glass.SM_SH_Door05_Glass" :`NewEnumerator4` "/Game/DoorsBPV2/Meshes/Doors/05/SM_MH_Door05_Glass.SM_MH_Door05_Glass" :`NewEnumerator5` "/Game/DoorsBPV2/Meshes/Doors/05/SM_LH_Door05_Glass.SM_LH_Door05_Glass" :!type "StaticMesh Object Reference")))

(fn `Get Door A`
  (params (Size :type "/Game/DoorsBPV2/Blueprints/Enums/Enum_SizeType Enum" :default "NewEnumerator0"))
  (returns (`Door Mesh` :type "StaticMesh Object Reference"))
  (return (select `/Game/DoorsBPV2/Blueprints/Enums/Enum_SizeType` Size :`NewEnumerator0` "/Game/DoorsBPV2/Meshes/Doors/A/SM_S_DoorA.SM_S_DoorA" :`NewEnumerator1` "/Game/DoorsBPV2/Meshes/Doors/A/SM_M_DoorA.SM_M_DoorA" :`NewEnumerator2` "/Game/DoorsBPV2/Meshes/Doors/A/SM_L_DoorA.SM_L_DoorA" :`NewEnumerator3` "/Game/DoorsBPV2/Meshes/Doors/A/SM_SH_DoorA.SM_SH_DoorA" :`NewEnumerator4` "/Game/DoorsBPV2/Meshes/Doors/A/SM_MH_DoorA.SM_MH_DoorA" :`NewEnumerator5` "/Game/DoorsBPV2/Meshes/Doors/A/SM_LH_DoorA.SM_LH_DoorA" :!type "StaticMesh Object Reference")))

(fn `Get Door B`
  (params (Size :type "/Game/DoorsBPV2/Blueprints/Enums/Enum_SizeType Enum" :default "NewEnumerator0"))
  (returns (`Door Mesh` :type "StaticMesh Object Reference"))
  (return (select `/Game/DoorsBPV2/Blueprints/Enums/Enum_SizeType` Size :`NewEnumerator0` "/Game/DoorsBPV2/Meshes/Doors/B/SM_S_DoorB.SM_S_DoorB" :`NewEnumerator1` "/Game/DoorsBPV2/Meshes/Doors/B/SM_M_DoorB.SM_M_DoorB" :`NewEnumerator2` "/Game/DoorsBPV2/Meshes/Doors/B/SM_L_DoorB.SM_L_DoorB" :`NewEnumerator3` "/Game/DoorsBPV2/Meshes/Doors/B/SM_SH_DoorB.SM_SH_DoorB" :`NewEnumerator4` "/Game/DoorsBPV2/Meshes/Doors/B/SM_MH_DoorB.SM_MH_DoorB" :`NewEnumerator5` "/Game/DoorsBPV2/Meshes/Doors/B/SM_LH_DoorB.SM_LH_DoorB" :!type "StaticMesh Object Reference")))

(fn `Get Door C`
  (params (Size :type "/Game/DoorsBPV2/Blueprints/Enums/Enum_SizeType Enum" :default "NewEnumerator0"))
  (returns (`Door Mesh` :type "StaticMesh Object Reference"))
  (return (select `/Game/DoorsBPV2/Blueprints/Enums/Enum_SizeType` Size :`NewEnumerator0` "/Game/DoorsBPV2/Meshes/Doors/C/SM_S_DoorC.SM_S_DoorC" :`NewEnumerator1` "/Game/DoorsBPV2/Meshes/Doors/C/SM_M_DoorC.SM_M_DoorC" :`NewEnumerator2` "/Game/DoorsBPV2/Meshes/Doors/C/SM_L_DoorC.SM_L_DoorC" :`NewEnumerator3` "/Game/DoorsBPV2/Meshes/Doors/C/SM_SH_DoorC.SM_SH_DoorC" :`NewEnumerator4` "/Game/DoorsBPV2/Meshes/Doors/C/SM_MH_DoorC.SM_MH_DoorC" :`NewEnumerator5` "/Game/DoorsBPV2/Meshes/Doors/C/SM_LH_DoorC.SM_LH_DoorC" :!type "StaticMesh Object Reference")))

(fn `Get Door D`
  (params (Size :type "/Game/DoorsBPV2/Blueprints/Enums/Enum_SizeType Enum" :default "NewEnumerator0"))
  (returns (`Door Mesh` :type "StaticMesh Object Reference"))
  (return (select `/Game/DoorsBPV2/Blueprints/Enums/Enum_SizeType` Size :`NewEnumerator0` "/Game/DoorsBPV2/Meshes/Doors/D/SM_S_DoorD.SM_S_DoorD" :`NewEnumerator1` "/Game/DoorsBPV2/Meshes/Doors/D/SM_M_DoorD.SM_M_DoorD" :`NewEnumerator2` "/Game/DoorsBPV2/Meshes/Doors/D/SM_L_DoorD.SM_L_DoorD" :`NewEnumerator3` "/Game/DoorsBPV2/Meshes/Doors/D/SM_SH_DoorD.SM_SH_DoorD" :`NewEnumerator4` "/Game/DoorsBPV2/Meshes/Doors/D/SM_MH_DoorD.SM_MH_DoorD" :`NewEnumerator5` "/Game/DoorsBPV2/Meshes/Doors/D/SM_LH_DoorD.SM_LH_DoorD" :!type "StaticMesh Object Reference")))

(fn `Get Door Details`
  (params (Size :type "/Game/DoorsBPV2/Blueprints/Enums/Enum_DoorSizes Enum" :default "NewEnumerator12"))
  (returns (DoorValues :type "/Game/DoorsBPV2/Blueprints/Structs/BPS_DoorSizes Structure"))
  (locals (`Door Size Structure` :type "Array of /Game/DoorsBPV2/Blueprints/Structs/BPS_DoorSizes Structure"))
  (bind _returnvalue (select `/Game/DoorsBPV2/Blueprints/Enums/Enum_DoorSizes` Size :`NewEnumerator12` 2040.0 :`NewEnumerator2` 2340.0 :`NewEnumerator9` 2040.0 :`NewEnumerator13` 2340.0 :`NewEnumerator15` 2040.0 :`NewEnumerator14` 2340.0 :`NewEnumerator0` 1972.0 :`NewEnumerator16` 2097.0 :`NewEnumerator28` 2347.0 :`NewEnumerator17` 1972.0 :`NewEnumerator18` 2097.0 :`NewEnumerator29` 2347.0 :`NewEnumerator19` 1972.0 :`NewEnumerator20` 2097.0 :`NewEnumerator30` 2347.0 :`NewEnumerator1` 2032.0 :`NewEnumerator6` 2134.0 :`NewEnumerator7` 2438.0 :`NewEnumerator11` 2032.0 :`NewEnumerator8` 2134.0 :`NewEnumerator10` 2438.0 :`NewEnumerator21` 2032.0 :`NewEnumerator22` 2134.0 :`NewEnumerator23` 2438.0 :`NewEnumerator24` 2040.0))
  (bind _returnvalue_2 (select `/Game/DoorsBPV2/Blueprints/Enums/Enum_DoorSizes` Size :`NewEnumerator12` "NewEnumerator0" :`NewEnumerator2` "NewEnumerator3" :`NewEnumerator9` "NewEnumerator1" :`NewEnumerator13` "NewEnumerator4" :`NewEnumerator15` "NewEnumerator2" :`NewEnumerator14` "NewEnumerator5" :`NewEnumerator0` "NewEnumerator0" :`NewEnumerator16` "NewEnumerator0" :`NewEnumerator28` "NewEnumerator3" :`NewEnumerator17` "NewEnumerator1" :`NewEnumerator18` "NewEnumerator1" :`NewEnumerator29` "NewEnumerator4" :`NewEnumerator19` "NewEnumerator2" :`NewEnumerator20` "NewEnumerator2" :`NewEnumerator30` "NewEnumerator5" :`NewEnumerator1` "NewEnumerator0" :`NewEnumerator6` "NewEnumerator0" :`NewEnumerator7` "NewEnumerator3" :`NewEnumerator11` "NewEnumerator1" :`NewEnumerator8` "NewEnumerator1" :`NewEnumerator10` "NewEnumerator4" :`NewEnumerator21` "NewEnumerator2" :`NewEnumerator22` "NewEnumerator2" :`NewEnumerator23` "NewEnumerator5" :`NewEnumerator24` "NewEnumerator1" :!type "/Game/DoorsBPV2/Blueprints/Enums/Enum_SizeType Enum"))
  (bind _returnvalue_3 (select `/Game/DoorsBPV2/Blueprints/Enums/Enum_DoorSizes` Size :`NewEnumerator12` 720.0 :`NewEnumerator2` 720.0 :`NewEnumerator9` 820.0 :`NewEnumerator13` 820.0 :`NewEnumerator15` 920.0 :`NewEnumerator14` 920.0 :`NewEnumerator0` 709.0 :`NewEnumerator16` 709.0 :`NewEnumerator28` 709.0 :`NewEnumerator17` 834.0 :`NewEnumerator18` 834.0 :`NewEnumerator29` 834.0 :`NewEnumerator19` 959.0 :`NewEnumerator20` 959.0 :`NewEnumerator30` 959.0 :`NewEnumerator1` 711.0 :`NewEnumerator6` 711.0 :`NewEnumerator7` 711.0 :`NewEnumerator11` 813.0 :`NewEnumerator8` 813.0 :`NewEnumerator10` 813.0 :`NewEnumerator21` 914.0 :`NewEnumerator22` 914.0 :`NewEnumerator23` 914.0 :`NewEnumerator24` 1.0))
  (bind _returnvalue_4 (/ _returnvalue (select `/Game/DoorsBPV2/Blueprints/Enums/Enum_SizeType` _returnvalue_2 :`NewEnumerator0` 2040.0 :`NewEnumerator1` 2040.0 :`NewEnumerator2` 2040.0 :`NewEnumerator3` 2340.0 :`NewEnumerator4` 2340.0 :`NewEnumerator5` 2340.0)))
  (bind _returnvalue_5 (/ _returnvalue_3 (select `/Game/DoorsBPV2/Blueprints/Enums/Enum_SizeType` _returnvalue_2 :`NewEnumerator0` 720.0 :`NewEnumerator1` 820.0 :`NewEnumerator2` 920.0 :`NewEnumerator3` 720.0 :`NewEnumerator4` 820.0 :`NewEnumerator5` 920.0)))
  (return (make `/Game/DoorsBPV2/Blueprints/Structs/BPS_DoorSizes` _returnvalue_2 (`KismetTextLibrary.Conv_TextToString` (`|FormatText` "Type {type}: {width} x {height} mm ({h} x {w})" (select `/Game/DoorsBPV2/Blueprints/Enums/Enum_SizeType` _returnvalue_2 :`NewEnumerator0` "S" :`NewEnumerator1` "M" :`NewEnumerator2` "L" :`NewEnumerator3` "SH" :`NewEnumerator4` "MH" :`NewEnumerator5` "LH" :!type "Text") _returnvalue_3 _returnvalue _returnvalue_5 _returnvalue_4)) _returnvalue_5 _returnvalue_4)))

(fn `Get Door E`
  (params (Size :type "/Game/DoorsBPV2/Blueprints/Enums/Enum_SizeType Enum" :default "NewEnumerator0"))
  (returns (`Door Mesh` :type "StaticMesh Object Reference"))
  (return (select `/Game/DoorsBPV2/Blueprints/Enums/Enum_SizeType` Size :`NewEnumerator0` "/Game/DoorsBPV2/Meshes/Doors/E/SM_S_DoorE.SM_S_DoorE" :`NewEnumerator1` "/Game/DoorsBPV2/Meshes/Doors/E/SM_M_DoorE.SM_M_DoorE" :`NewEnumerator2` "/Game/DoorsBPV2/Meshes/Doors/E/SM_L_DoorE.SM_L_DoorE" :`NewEnumerator3` "/Game/DoorsBPV2/Meshes/Doors/E/SM_SH_DoorE.SM_SH_DoorE" :`NewEnumerator4` "/Game/DoorsBPV2/Meshes/Doors/E/SM_MH_DoorE.SM_MH_DoorE" :`NewEnumerator5` "/Game/DoorsBPV2/Meshes/Doors/E/SM_LH_DoorE.SM_LH_DoorE" :!type "StaticMesh Object Reference")))

(fn `Get Door Meshes`
  (params (Size :type "/Game/DoorsBPV2/Blueprints/Enums/Enum_SizeType Enum" :default "NewEnumerator0") (Style :type "/Game/DoorsBPV2/Blueprints/Enums/Enum_DoorType Enum" :default "NewEnumerator0"))
  (returns (Door :type "StaticMesh Object Reference") (Glass :type "StaticMesh Object Reference") (`Glass Mesh` :type Boolean))
  (bind (_door_mesh _glass_mesh) (`self.Get Door 04` Size))
  (bind (_door_mesh_2 _glass_mesh_2) (`self.Get Door 05` Size))
  (return (select `/Game/DoorsBPV2/Blueprints/Enums/Enum_DoorType` Style :`NewEnumerator0` (`self.Get Door A` Size) :`NewEnumerator7` (`self.Get Door D` Size) :`NewEnumerator1` (`self.Get Door B` Size) :`NewEnumerator2` (`self.Get Door C` Size) :`NewEnumerator4` (`self.Get Door E` Size) :`NewEnumerator5` _door_mesh :`NewEnumerator6` _door_mesh_2 :`NewEnumerator9` (`self.Get Glass Door` Size)) (select `/Game/DoorsBPV2/Blueprints/Enums/Enum_DoorType` Style :`NewEnumerator0` "/Game/DoorsBPV2/Meshes/Doors/SM_DoorX_Glass.SM_DoorX_Glass" :`NewEnumerator7` "/Game/DoorsBPV2/Meshes/Doors/SM_DoorX_Glass.SM_DoorX_Glass" :`NewEnumerator1` "/Game/DoorsBPV2/Meshes/Doors/SM_DoorX_Glass.SM_DoorX_Glass" :`NewEnumerator2` "/Game/DoorsBPV2/Meshes/Doors/SM_DoorX_Glass.SM_DoorX_Glass" :`NewEnumerator4` "/Game/DoorsBPV2/Meshes/Doors/SM_DoorX_Glass.SM_DoorX_Glass" :`NewEnumerator5` _glass_mesh :`NewEnumerator6` _glass_mesh_2) (select `/Game/DoorsBPV2/Blueprints/Enums/Enum_DoorType` Style :`NewEnumerator5` true :`NewEnumerator6` true)))

(fn `Get Door or Custom Meshes`
  (params (Size :type "/Game/DoorsBPV2/Blueprints/Enums/Enum_SizeType Enum" :default "NewEnumerator0") (Type :type "/Game/DoorsBPV2/Blueprints/Enums/Enum_DoorType Enum" :default "NewEnumerator8") (`Custom Door` :type "StaticMesh Object Reference") (`Custom Glass` :type "StaticMesh Object Reference"))
  (returns (Door :type "StaticMesh Object Reference") (Glass :type "StaticMesh Object Reference"))
  (bind (_door _glass) (`self.Get Door Meshes` Size Type))
  (if (`|EnumInequality` Type "NewEnumerator8")
    (return `Custom Door` `Custom Glass`)
    (else
      (return _door _glass))))

(fn `Get Door Size Offsets`
  (params (Size :type "/Game/DoorsBPV2/Blueprints/Enums/Enum_DoorSizes Enum" :default "NewEnumerator12") (`Handle Horizontal Offset` :type "Float (double-precision)"))
  (returns (DoorOffset :type "Float (double-precision)") (HandleOffset :type "Float (double-precision)") (TopHeightOffset :type "Float (double-precision)") (`Shutter Offset` :type "Float (double-precision)"))
  (bind _size (break `/Game/DoorsBPV2/Blueprints/Structs/BPS_DoorSizes` (`self.Get Door Details` Size)))
  (return (select `/Game/DoorsBPV2/Blueprints/Enums/Enum_SizeType` _size :`NewEnumerator0` 5.0 :`NewEnumerator2` -5.0 :`NewEnumerator3` 5.0 :`NewEnumerator5` -5.0) (- (select `/Game/DoorsBPV2/Blueprints/Enums/Enum_SizeType` _size :`NewEnumerator0` 72.0 :`NewEnumerator1` 82.0 :`NewEnumerator2` 92.0 :`NewEnumerator3` 72.0 :`NewEnumerator4` 82.0 :`NewEnumerator5` 92.0) `Handle Horizontal Offset`) (select `/Game/DoorsBPV2/Blueprints/Enums/Enum_SizeType` _size :`NewEnumerator3` 30.0 :`NewEnumerator4` 30.0 :`NewEnumerator5` 30.0) (- `Handle Horizontal Offset` 6.0)))

(fn `Get Frame A`
  (params (Size :type "/Game/DoorsBPV2/Blueprints/Enums/Enum_SizeType Enum" :default "NewEnumerator0") (`Is Double` :type Boolean))
  (returns (NewParam :type "StaticMesh Object Reference"))
  (return (select `bool` `Is Double` :`false` (select `/Game/DoorsBPV2/Blueprints/Enums/Enum_SizeType` Size :`NewEnumerator0` "/Game/DoorsBPV2/Meshes/Frames/A/SM_S_FrameA.SM_S_FrameA" :`NewEnumerator1` "/Game/DoorsBPV2/Meshes/Frames/A/SM_M_FrameA.SM_M_FrameA" :`NewEnumerator2` "/Game/DoorsBPV2/Meshes/Frames/A/SM_L_FrameA.SM_L_FrameA" :`NewEnumerator3` "/Game/DoorsBPV2/Meshes/Frames/A/SM_SH_FrameA.SM_SH_FrameA" :`NewEnumerator4` "/Game/DoorsBPV2/Meshes/Frames/A/SM_MH_FrameA.SM_MH_FrameA" :`NewEnumerator5` "/Game/DoorsBPV2/Meshes/Frames/A/SM_LH_FrameA.SM_LH_FrameA" :!type "StaticMesh Object Reference") :`true` (select `/Game/DoorsBPV2/Blueprints/Enums/Enum_SizeType` Size :`NewEnumerator0` "/Game/DoorsBPV2/Meshes/Frames/A/SM_S2_FrameA.SM_S2_FrameA" :`NewEnumerator1` "/Game/DoorsBPV2/Meshes/Frames/A/SM_M2_FrameA.SM_M2_FrameA" :`NewEnumerator2` "/Game/DoorsBPV2/Meshes/Frames/A/SM_L2_FrameA.SM_L2_FrameA" :`NewEnumerator3` "/Game/DoorsBPV2/Meshes/Frames/A/SM_SH2_FrameA.SM_SH2_FrameA" :`NewEnumerator4` "/Game/DoorsBPV2/Meshes/Frames/A/SM_MH2_FrameA.SM_MH2_FrameA" :`NewEnumerator5` "/Game/DoorsBPV2/Meshes/Frames/A/SM_LH2_FrameA.SM_LH2_FrameA" :!type "StaticMesh Object Reference"))))

(fn `Get Frame B`
  (params (Size :type "/Game/DoorsBPV2/Blueprints/Enums/Enum_SizeType Enum" :default "NewEnumerator0") (`Is Double` :type Boolean))
  (returns (NewParam :type "StaticMesh Object Reference"))
  (return (select `bool` `Is Double` :`false` (select `/Game/DoorsBPV2/Blueprints/Enums/Enum_SizeType` Size :`NewEnumerator0` "/Game/DoorsBPV2/Meshes/Frames/B/SM_S_FrameB.SM_S_FrameB" :`NewEnumerator1` "/Game/DoorsBPV2/Meshes/Frames/B/SM_M_FrameB.SM_M_FrameB" :`NewEnumerator2` "/Game/DoorsBPV2/Meshes/Frames/B/SM_L_FrameB.SM_L_FrameB" :`NewEnumerator3` "/Game/DoorsBPV2/Meshes/Frames/B/SM_SH_FrameB.SM_SH_FrameB" :`NewEnumerator4` "/Game/DoorsBPV2/Meshes/Frames/B/SM_MH_FrameB.SM_MH_FrameB" :`NewEnumerator5` "/Game/DoorsBPV2/Meshes/Frames/B/SM_LH_FrameB.SM_LH_FrameB" :!type "StaticMesh Object Reference") :`true` (select `/Game/DoorsBPV2/Blueprints/Enums/Enum_SizeType` Size :`NewEnumerator0` "/Game/DoorsBPV2/Meshes/Frames/B/SM_S2_FrameB.SM_S2_FrameB" :`NewEnumerator1` "/Game/DoorsBPV2/Meshes/Frames/B/SM_M2_FrameB.SM_M2_FrameB" :`NewEnumerator2` "/Game/DoorsBPV2/Meshes/Frames/B/SM_L2_FrameB.SM_L2_FrameB" :`NewEnumerator3` "/Game/DoorsBPV2/Meshes/Frames/B/SM_SH2_FrameB.SM_SH2_FrameB" :`NewEnumerator4` "/Game/DoorsBPV2/Meshes/Frames/B/SM_MH2_FrameB.SM_MH2_FrameB" :`NewEnumerator5` "/Game/DoorsBPV2/Meshes/Frames/B/SM_LH2_FrameB.SM_LH2_FrameB" :!type "StaticMesh Object Reference"))))

(fn `Get Frame C`
  (params (Size :type "/Game/DoorsBPV2/Blueprints/Enums/Enum_SizeType Enum" :default "NewEnumerator0") (`Is Double` :type Boolean))
  (returns (NewParam :type "StaticMesh Object Reference"))
  (return (select `bool` `Is Double` :`false` (select `/Game/DoorsBPV2/Blueprints/Enums/Enum_SizeType` Size :`NewEnumerator0` "/Game/DoorsBPV2/Meshes/Frames/C/SM_S_FrameC.SM_S_FrameC" :`NewEnumerator1` "/Game/DoorsBPV2/Meshes/Frames/C/SM_M_FrameC.SM_M_FrameC" :`NewEnumerator2` "/Game/DoorsBPV2/Meshes/Frames/C/SM_L_FrameC.SM_L_FrameC" :`NewEnumerator3` "/Game/DoorsBPV2/Meshes/Frames/C/SM_SH_FrameC.SM_SH_FrameC" :`NewEnumerator4` "/Game/DoorsBPV2/Meshes/Frames/C/SM_MH_FrameC.SM_MH_FrameC" :`NewEnumerator5` "/Game/DoorsBPV2/Meshes/Frames/C/SM_LH_FrameC.SM_LH_FrameC" :!type "StaticMesh Object Reference") :`true` (select `/Game/DoorsBPV2/Blueprints/Enums/Enum_SizeType` Size :`NewEnumerator0` "/Game/DoorsBPV2/Meshes/Frames/C/SM_S2_FrameC.SM_S2_FrameC" :`NewEnumerator1` "/Game/DoorsBPV2/Meshes/Frames/C/SM_M2_FrameC.SM_M2_FrameC" :`NewEnumerator2` "/Game/DoorsBPV2/Meshes/Frames/C/SM_L2_FrameC.SM_L2_FrameC" :`NewEnumerator3` "/Game/DoorsBPV2/Meshes/Frames/C/SM_SH2_FrameC.SM_SH2_FrameC" :`NewEnumerator4` "/Game/DoorsBPV2/Meshes/Frames/C/SM_MH2_FrameC.SM_MH2_FrameC" :`NewEnumerator5` "/Game/DoorsBPV2/Meshes/Frames/C/SM_LH2_FrameC.SM_LH2_FrameC" :!type "StaticMesh Object Reference"))))

(fn `Get Frame D`
  (params (Size :type "/Game/DoorsBPV2/Blueprints/Enums/Enum_SizeType Enum" :default "NewEnumerator0") (`Is Double` :type Boolean))
  (returns (NewParam :type "StaticMesh Object Reference"))
  (return (select `bool` `Is Double` :`false` (select `/Game/DoorsBPV2/Blueprints/Enums/Enum_SizeType` Size :`NewEnumerator0` "/Game/DoorsBPV2/Meshes/Frames/D/SM_S_FrameD.SM_S_FrameD" :`NewEnumerator1` "/Game/DoorsBPV2/Meshes/Frames/D/SM_M_FrameD.SM_M_FrameD" :`NewEnumerator2` "/Game/DoorsBPV2/Meshes/Frames/D/SM_L_FrameD.SM_L_FrameD" :`NewEnumerator3` "/Game/DoorsBPV2/Meshes/Frames/D/SM_SH_FrameD.SM_SH_FrameD" :`NewEnumerator4` "/Game/DoorsBPV2/Meshes/Frames/D/SM_MH_FrameD.SM_MH_FrameD" :`NewEnumerator5` "/Game/DoorsBPV2/Meshes/Frames/D/SM_LH_FrameD.SM_LH_FrameD" :!type "StaticMesh Object Reference") :`true` (select `/Game/DoorsBPV2/Blueprints/Enums/Enum_SizeType` Size :`NewEnumerator0` "/Game/DoorsBPV2/Meshes/Frames/D/SM_S2_FrameD.SM_S2_FrameD" :`NewEnumerator1` "/Game/DoorsBPV2/Meshes/Frames/D/SM_M2_FrameD.SM_M2_FrameD" :`NewEnumerator2` "/Game/DoorsBPV2/Meshes/Frames/D/SM_L2_FrameD.SM_L2_FrameD" :`NewEnumerator3` "/Game/DoorsBPV2/Meshes/Frames/D/SM_SH2_FrameD.SM_SH2_FrameD" :`NewEnumerator4` "/Game/DoorsBPV2/Meshes/Frames/D/SM_MH2_FrameD.SM_MH2_FrameD" :`NewEnumerator5` "/Game/DoorsBPV2/Meshes/Frames/D/SM_LH2_FrameD.SM_LH2_FrameD" :!type "StaticMesh Object Reference"))))

(fn `Get Frame Mesh`
  (params (Type :type "/Game/DoorsBPV2/Blueprints/Enums/Enum_FrameType Enum" :default "NewEnumerator0") (Size :type "/Game/DoorsBPV2/Blueprints/Enums/Enum_SizeType Enum" :default "NewEnumerator0") (isDouble :type Boolean))
  (returns (`Frame Mesh` :type "StaticMesh Object Reference") (`Door Pos Y Offset` :type "Float (double-precision)"))
  (return (select `/Game/DoorsBPV2/Blueprints/Enums/Enum_FrameType` Type :`NewEnumerator0` (`self.Get Frame A` Size isDouble) :`NewEnumerator1` (`self.Get Frame B` Size isDouble) :`NewEnumerator2` (`self.Get Frame C` Size isDouble) :`NewEnumerator4` (`self.Get Frame D` Size isDouble)) (select `/Game/DoorsBPV2/Blueprints/Enums/Enum_FrameType` Type :`NewEnumerator1` -1.0 :`NewEnumerator4` -1.0)))

(fn `Get Frame Transform`
  (params (BPS_DoorSizes :type "/Game/DoorsBPV2/Blueprints/Structs/BPS_DoorSizes Structure (by ref)") (Flipped :type Boolean) (`Thickness Scale` :type "Float (double-precision)" :default 1.0))
  (returns (`Universal Scale` :type "Vector Structure") (Transform :type "Transform Structure"))
  (bind (_size _note _scalewidth _scaleheight) (break `/Game/DoorsBPV2/Blueprints/Structs/BPS_DoorSizes` BPS_DoorSizes))
  (bind _returnvalue (`KismetMathLibrary.MakeVector` `Thickness Scale` (select `bool` Flipped :`false` (* -1.0 _scalewidth) :`true` _scalewidth) _scaleheight))
  (return _returnvalue (`KismetMathLibrary.MakeTransform` (0.0 0.0 0.0) (struct) _returnvalue)))

(fn `Get Frame X`
  (params (Size :type "/Game/DoorsBPV2/Blueprints/Enums/Enum_SizeType Enum" :default "NewEnumerator0") (`Is Double` :type Boolean))
  (returns (NewParam :type "StaticMesh Object Reference"))
  (return (select `bool` `Is Double` :`false` (select `/Game/DoorsBPV2/Blueprints/Enums/Enum_SizeType` Size :!type "StaticMesh Object Reference") :`true` (select `/Game/DoorsBPV2/Blueprints/Enums/Enum_SizeType` Size :!type "StaticMesh Object Reference"))))

(fn `Get Glass Door`
  (params (Size :type "/Game/DoorsBPV2/Blueprints/Enums/Enum_SizeType Enum" :default "NewEnumerator0"))
  (returns (`Door Mesh` :type "StaticMesh Object Reference"))
  (return (select `/Game/DoorsBPV2/Blueprints/Enums/Enum_SizeType` Size :`NewEnumerator0` "/Game/DoorsBPV2/Meshes/Doors/Glass/SM_S_GlassDoor01.SM_S_GlassDoor01" :`NewEnumerator1` "/Game/DoorsBPV2/Meshes/Doors/Glass/SM_M_GlassDoor01.SM_M_GlassDoor01" :`NewEnumerator2` "/Game/DoorsBPV2/Meshes/Doors/Glass/SM_L_GlassDoor01.SM_L_GlassDoor01" :`NewEnumerator3` "/Game/DoorsBPV2/Meshes/Doors/Glass/SM_SH_GlassDoor01.SM_SH_GlassDoor01" :`NewEnumerator4` "/Game/DoorsBPV2/Meshes/Doors/Glass/SM_MH_GlassDoor01.SM_MH_GlassDoor01" :`NewEnumerator5` "/Game/DoorsBPV2/Meshes/Doors/Glass/SM_LH_GlassDoor01.SM_LH_GlassDoor01" :!type "StaticMesh Object Reference")))

(fn `Get Handle Unscale Height`
  (params (Size :type "/Game/DoorsBPV2/Blueprints/Enums/Enum_DoorSizes Enum" :default "NewEnumerator12") (`Handle Height ` :type "Float (double-precision)") (`Lock Plate Offset` :type "Float (double-precision)"))
  (returns (`Scaled Height` :type "Float (double-precision)") (`Scaled Lock Offset` :type "Float (double-precision)"))
  (bind (_size _note _scalewidth _scaleheight) (break `/Game/DoorsBPV2/Blueprints/Structs/BPS_DoorSizes` (`self.Get Door Details` Size)))
  (return (/ `Handle Height ` _scaleheight) (/ `Lock Plate Offset` _scaleheight)))

(fn `Get SFrame A`
  (params (Size :type "/Game/DoorsBPV2/Blueprints/Enums/Enum_SizeType Enum" :default "NewEnumerator0") (`Is Double` :type Boolean))
  (returns (NewParam :type "StaticMesh Object Reference"))
  (return (select `bool` `Is Double` :`false` (select `/Game/DoorsBPV2/Blueprints/Enums/Enum_SizeType` Size :`NewEnumerator0` "/Game/DoorsBPV2/Meshes/Frames/AS/SM_S_SFrameA.SM_S_SFrameA" :`NewEnumerator1` "/Game/DoorsBPV2/Meshes/Frames/AS/SM_M_SFrameA.SM_M_SFrameA" :`NewEnumerator2` "/Game/DoorsBPV2/Meshes/Frames/AS/SM_L_SFrameA.SM_L_SFrameA" :`NewEnumerator3` "/Game/DoorsBPV2/Meshes/Frames/AS/SM_SH_SFrameA.SM_SH_SFrameA" :`NewEnumerator4` "/Game/DoorsBPV2/Meshes/Frames/AS/SM_MH_SFrameA.SM_MH_SFrameA" :`NewEnumerator5` "/Game/DoorsBPV2/Meshes/Frames/AS/SM_LH_SFrameA.SM_LH_SFrameA" :!type "StaticMesh Object Reference") :`true` (select `/Game/DoorsBPV2/Blueprints/Enums/Enum_SizeType` Size :`NewEnumerator0` "/Game/DoorsBPV2/Meshes/Frames/AS/SM_S2_SFrameA.SM_S2_SFrameA" :`NewEnumerator1` "/Game/DoorsBPV2/Meshes/Frames/AS/SM_M2_SFrameA.SM_M2_SFrameA" :`NewEnumerator2` "/Game/DoorsBPV2/Meshes/Frames/AS/SM_L2_SFrameA.SM_L2_SFrameA" :`NewEnumerator3` "/Game/DoorsBPV2/Meshes/Frames/AS/SM_SH2_SFrameA.SM_SH2_SFrameA" :`NewEnumerator4` "/Game/DoorsBPV2/Meshes/Frames/AS/SM_MH2_SFrameA.SM_MH2_SFrameA" :`NewEnumerator5` "/Game/DoorsBPV2/Meshes/Frames/AS/SM_LH2_SFrameA.SM_LH2_SFrameA" :!type "StaticMesh Object Reference"))))

(fn `Get SFrame B`
  (params (Size :type "/Game/DoorsBPV2/Blueprints/Enums/Enum_SizeType Enum" :default "NewEnumerator0") (`Is Double` :type Boolean))
  (returns (NewParam :type "StaticMesh Object Reference"))
  (return (select `bool` `Is Double` :`false` (select `/Game/DoorsBPV2/Blueprints/Enums/Enum_SizeType` Size :`NewEnumerator0` "/Game/DoorsBPV2/Meshes/Frames/BS/SM_S_SFrameB.SM_S_SFrameB" :`NewEnumerator1` "/Game/DoorsBPV2/Meshes/Frames/BS/SM_M_SFrameB.SM_M_SFrameB" :`NewEnumerator2` "/Game/DoorsBPV2/Meshes/Frames/BS/SM_L_SFrameB.SM_L_SFrameB" :`NewEnumerator3` "/Game/DoorsBPV2/Meshes/Frames/BS/SM_SH_SFrameB.SM_SH_SFrameB" :`NewEnumerator4` "/Game/DoorsBPV2/Meshes/Frames/BS/SM_MH_SFrameB.SM_MH_SFrameB" :`NewEnumerator5` "/Game/DoorsBPV2/Meshes/Frames/BS/SM_LH_SFrameB.SM_LH_SFrameB" :!type "StaticMesh Object Reference") :`true` (select `/Game/DoorsBPV2/Blueprints/Enums/Enum_SizeType` Size :`NewEnumerator0` "/Game/DoorsBPV2/Meshes/Frames/BS/SM_S2_SFrameB.SM_S2_SFrameB" :`NewEnumerator1` "/Game/DoorsBPV2/Meshes/Frames/BS/SM_M2_SFrameB.SM_M2_SFrameB" :`NewEnumerator2` "/Game/DoorsBPV2/Meshes/Frames/BS/SM_L2_SFrameB.SM_L2_SFrameB" :`NewEnumerator3` "/Game/DoorsBPV2/Meshes/Frames/BS/SM_SH2_SFrameB.SM_SH2_SFrameB" :`NewEnumerator4` "/Game/DoorsBPV2/Meshes/Frames/BS/SM_MH2_SFrameB.SM_MH2_SFrameB" :`NewEnumerator5` "/Game/DoorsBPV2/Meshes/Frames/BS/SM_LH2_SFrameB.SM_LH2_SFrameB" :!type "StaticMesh Object Reference"))))

(fn `Get SFrame C`
  (params (Size :type "/Game/DoorsBPV2/Blueprints/Enums/Enum_SizeType Enum" :default "NewEnumerator0") (`Is Double` :type Boolean))
  (returns (NewParam :type "StaticMesh Object Reference"))
  (return (select `bool` `Is Double` :`false` (select `/Game/DoorsBPV2/Blueprints/Enums/Enum_SizeType` Size :`NewEnumerator0` "/Game/DoorsBPV2/Meshes/Frames/CS/SM_S_SFrameC.SM_S_SFrameC" :`NewEnumerator1` "/Game/DoorsBPV2/Meshes/Frames/CS/SM_M_SFrameC.SM_M_SFrameC" :`NewEnumerator2` "/Game/DoorsBPV2/Meshes/Frames/CS/SM_L_SFrameC.SM_L_SFrameC" :`NewEnumerator3` "/Game/DoorsBPV2/Meshes/Frames/CS/SM_SH_SFrameC.SM_SH_SFrameC" :`NewEnumerator4` "/Game/DoorsBPV2/Meshes/Frames/CS/SM_MH_SFrameC.SM_MH_SFrameC" :`NewEnumerator5` "/Game/DoorsBPV2/Meshes/Frames/CS/SM_LH_SFrameC.SM_LH_SFrameC" :!type "StaticMesh Object Reference") :`true` (select `/Game/DoorsBPV2/Blueprints/Enums/Enum_SizeType` Size :`NewEnumerator0` "/Game/DoorsBPV2/Meshes/Frames/CS/SM_S2_SFrameC.SM_S2_SFrameC" :`NewEnumerator1` "/Game/DoorsBPV2/Meshes/Frames/CS/SM_M2_SFrameC.SM_M2_SFrameC" :`NewEnumerator2` "/Game/DoorsBPV2/Meshes/Frames/CS/SM_L2_SFrameC.SM_L2_SFrameC" :`NewEnumerator3` "/Game/DoorsBPV2/Meshes/Frames/CS/SM_SH2_SFrameC.SM_SH2_SFrameC" :`NewEnumerator4` "/Game/DoorsBPV2/Meshes/Frames/CS/SM_MH2_SFrameC.SM_MH2_SFrameC" :`NewEnumerator5` "/Game/DoorsBPV2/Meshes/Frames/CS/SM_LH2_SFrameC.SM_LH2_SFrameC" :!type "StaticMesh Object Reference"))))

(fn `Get SFrame Mesh`
  (params (Type :type "/Game/DoorsBPV2/Blueprints/Enums/Enum_FrameType Enum" :default "NewEnumerator0") (Size :type "/Game/DoorsBPV2/Blueprints/Enums/Enum_SizeType Enum" :default "NewEnumerator0") (isDouble :type Boolean))
  (returns (`SD Frame Mesh` :type "StaticMesh Object Reference"))
  (bind _newparam (`self.Get SFrame A` Size isDouble))
  (return (select `/Game/DoorsBPV2/Blueprints/Enums/Enum_FrameType` Type :`NewEnumerator0` _newparam :`NewEnumerator1` (`self.Get SFrame B` Size isDouble) :`NewEnumerator2` (`self.Get SFrame C` Size isDouble) :`NewEnumerator4` _newparam)))

(fn `Get SFrame X`
  (params (Size :type "/Game/DoorsBPV2/Blueprints/Enums/Enum_SizeType Enum" :default "NewEnumerator0") (`Is Double` :type Boolean))
  (returns (NewParam :type "StaticMesh Object Reference"))
  (return (select `bool` `Is Double` :`false` (select `/Game/DoorsBPV2/Blueprints/Enums/Enum_SizeType` Size :!type "StaticMesh Object Reference") :`true` (select `/Game/DoorsBPV2/Blueprints/Enums/Enum_SizeType` Size :!type "StaticMesh Object Reference"))))

(fn `Get Text Transform`
  (params (Location :type "Vector Structure") (Orientation :type Boolean))
  (returns (Transform :type "Transform Structure"))
  (return (`KismetMathLibrary.MakeTransform` Location (select `bool` Orientation :`true` (struct :`Yaw` 180.0) :!type "Rotator Structure"))))

(fn `Get Top Frame Mesh`
  (params (Type :type "/Game/DoorsBPV2/Blueprints/Enums/Enum_FrameType Enum" :default "NewEnumerator0") (Size :type "/Game/DoorsBPV2/Blueprints/Enums/Enum_SizeType Enum" :default "NewEnumerator0"))
  (returns (`Top Frame` :type "StaticMesh Object Reference") (`Top Frame Glass` :type "StaticMesh Object Reference"))
  (bind _returnvalue (select `/Game/DoorsBPV2/Blueprints/Enums/Enum_SizeType` Size :`NewEnumerator0` "/Game/DoorsBPV2/Meshes/Frames/A/SM_S_FrameA_Top.SM_S_FrameA_Top" :`NewEnumerator1` "/Game/DoorsBPV2/Meshes/Frames/A/SM_M_FrameA_Top.SM_M_FrameA_Top" :`NewEnumerator2` "/Game/DoorsBPV2/Meshes/Frames/A/SM_L_FrameA_Top.SM_L_FrameA_Top" :`NewEnumerator3` "/Game/DoorsBPV2/Meshes/Frames/A/SM_S_FrameA_Top.SM_S_FrameA_Top" :`NewEnumerator4` "/Game/DoorsBPV2/Meshes/Frames/A/SM_M_FrameA_Top.SM_M_FrameA_Top" :`NewEnumerator5` "/Game/DoorsBPV2/Meshes/Frames/A/SM_L_FrameA_Top.SM_L_FrameA_Top" :!type "StaticMesh Object Reference"))
  (bind _returnvalue_2 (select `/Game/DoorsBPV2/Blueprints/Enums/Enum_SizeType` Size :`NewEnumerator0` "/Game/DoorsBPV2/Meshes/Frames/A/SM_S_FrameA_TopGlass.SM_S_FrameA_TopGlass" :`NewEnumerator1` "/Game/DoorsBPV2/Meshes/Frames/A/SM_M_FrameA_TopGlass.SM_M_FrameA_TopGlass" :`NewEnumerator2` "/Game/DoorsBPV2/Meshes/Frames/A/SM_L_FrameA_TopGlass.SM_L_FrameA_TopGlass" :`NewEnumerator3` "/Game/DoorsBPV2/Meshes/Frames/A/SM_S_FrameA_TopGlass.SM_S_FrameA_TopGlass" :`NewEnumerator4` "/Game/DoorsBPV2/Meshes/Frames/A/SM_M_FrameA_TopGlass.SM_M_FrameA_TopGlass" :`NewEnumerator5` "/Game/DoorsBPV2/Meshes/Frames/A/SM_L_FrameA_TopGlass.SM_L_FrameA_TopGlass" :!type "StaticMesh Object Reference"))
  (return (select `/Game/DoorsBPV2/Blueprints/Enums/Enum_FrameType` Type :`NewEnumerator0` _returnvalue :`NewEnumerator1` _returnvalue :`NewEnumerator2` _returnvalue) (select `/Game/DoorsBPV2/Blueprints/Enums/Enum_FrameType` Type :`NewEnumerator0` _returnvalue_2 :`NewEnumerator1` _returnvalue_2 :`NewEnumerator2` _returnvalue_2)))

(fn `Get Top Transform`
  (params (`Top Pos` :type "Float (double-precision)") (`Window Z Offset` :type "Float (double-precision)") (`Window Z Scale` :type "Float (double-precision)") (`Size Type` :type "/Game/DoorsBPV2/Blueprints/Enums/Enum_SizeType Enum" :default "NewEnumerator1") (`Double Doors` :type Boolean) (`Door 2` :type Boolean))
  (returns (Transform :type "Transform Structure"))
  (bind _returnvalue (/ 79.0 86.0))
  (bind _returnvalue_2 (/ 89.0 96.0))
  (bind _returnvalue_3 (/ 99.0 106.0))
  (return (`KismetMathLibrary.MakeTransform` (`KismetMathLibrary.MakeVector` 0.0 (select `bool` `Double Doors` :`true` (select `bool` `Door 2` :`false` -3.5 :`true` (select `/Game/DoorsBPV2/Blueprints/Enums/Enum_SizeType` `Size Type` :`NewEnumerator0` 75.8 :`NewEnumerator1` 85.8 :`NewEnumerator2` 95.8 :`NewEnumerator3` 75.75 :`NewEnumerator4` 85.75 :`NewEnumerator5` 95.75))) (+ `Top Pos` `Window Z Offset` 212.2)) (struct) (`KismetMathLibrary.MakeVector` 1.0 (select `bool` `Double Doors` :`false` 1.0 :`true` (select `/Game/DoorsBPV2/Blueprints/Enums/Enum_SizeType` `Size Type` :`NewEnumerator0` _returnvalue :`NewEnumerator1` _returnvalue_2 :`NewEnumerator2` _returnvalue_3 :`NewEnumerator3` _returnvalue :`NewEnumerator4` _returnvalue_2 :`NewEnumerator5` _returnvalue_3)) `Window Z Scale`))))

(fn `GetCustomOffset`
  (params (DoorMesh :type "StaticMesh Object Reference") (`Rotation Z` :type "/Game/DoorsBPV2/Blueprints/Enums/Enum_Rotation Enum" :default "NewEnumerator0") (Scale :type "Vector Structure"))
  (returns (Offset :type "Vector Structure"))
  (bind _x (.x Scale))
  (bind _y (.y Scale))
  (bind (_origin _boxextent) (`KismetMathLibrary.BreakBoxSphereBounds` (`StaticMesh.GetBounds` DoorMesh)))
  (bind _x_2 (.x _origin))
  (bind _y_2 (.y _origin))
  (bind _x_3 (.x _boxextent))
  (bind _y_3 (.y _boxextent))
  (bind _returnvalue (* _x_2 _x))
  (bind _returnvalue_2 (* _y_2 _y))
  (bind _returnvalue_3 (* (select `/Game/DoorsBPV2/Blueprints/Enums/Enum_Rotation` `Rotation Z` :`NewEnumerator0` (- _y_2 _y_3) :`NewEnumerator1` (- _x_2 _x_3) :`NewEnumerator2` (+ _y_2 _y_3) :`NewEnumerator3` (+ _x_2 _x_3)) (select `/Game/DoorsBPV2/Blueprints/Enums/Enum_Rotation` `Rotation Z` :`NewEnumerator0` _y :`NewEnumerator1` _x :`NewEnumerator2` _y :`NewEnumerator3` _x) -1.0))
  (return (`KismetMathLibrary.MakeVector` (select `/Game/DoorsBPV2/Blueprints/Enums/Enum_Rotation` `Rotation Z` :`NewEnumerator0` (- -2.0 _returnvalue) :`NewEnumerator1` _returnvalue_3 :`NewEnumerator2` (- 2.0 _returnvalue) :`NewEnumerator3` _returnvalue_3) (select `/Game/DoorsBPV2/Blueprints/Enums/Enum_Rotation` `Rotation Z` :`NewEnumerator0` _returnvalue_3 :`NewEnumerator1` (- 2.0 _returnvalue_2) :`NewEnumerator2` _returnvalue_3 :`NewEnumerator3` (- -2.0 _returnvalue_2)) (* (.z Scale) (- (.z _boxextent) (.z _origin))))))

(fn `Mirror to Entry Side`
  (params (InTransform :type "Transform Structure (by ref)"))
  (returns (`Mirrored X` :type "Transform Structure"))
  (return (`KismetMathLibrary.MakeTransform` (`KismetMathLibrary.MakeVector` (+ (.x (.location InTransform)) -4.0) 0.0 (.z (.location InTransform))) (.rotation InTransform) (`KismetMathLibrary.MakeVector` (* (.x (.scale InTransform)) -1.0) (.y (.scale InTransform)) (.z (.scale InTransform))))))