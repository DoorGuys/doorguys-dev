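; BP_DoorController is a keyboard-driven controller that broadcasts interaction and variation changes to doors.
; Pressing R sends InteractMessage to every actor implementing BPI_Doors_Interaction.
; Number keys call SetVariation, which broadcasts a variation ID and tag through the same interface, covering three variations for each of two tags.
; Each broadcast gathers actors with GetAllActorsWithInterface at press time, so no door references are stored.
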(event `Key|R`
  (params (Key :type "Key Structure"))
  ;[0.3802 0.4758 1 0.5] Interaction
  (:`Pressed`
    (bind _outactors (`GameplayStatics.GetAllActorsWithInterface` "/Game/DoorsBPV2/Blueprints/Others/BPI_Doors_Interaction.BPI_Doors_Interaction_C"))
    (for _array_element _outactors
      (message `/Game/DoorsBPV2/Blueprints/Others/BPI_Doors_Interaction.Interact` _array_element))))

(event `Set Variation`
  (params (ID :type Integer) (Tag :type String))
  ;[1 1 1 0.5] Variation
  (bind _outactors (`GameplayStatics.GetAllActorsWithInterface` "/Game/DoorsBPV2/Blueprints/Others/BPI_Doors_Interaction.BPI_Doors_Interaction_C"))
  (for _array_element _outactors
    (message `/Game/DoorsBPV2/Blueprints/Others/BPI_Doors_Interaction.Change Var ID` _array_element ID Tag)))

(event `Key|One`
  (params (Key :type "Key Structure"))
  ;[0.5875 0.1352 1 0.5] Tag 1
  (:`Pressed`
    (`self.Set Variation` 0 (`self.Tag1`))))

(event `Key|Four`
  (params (Key :type "Key Structure"))
  ;[0.5875 0.1352 1 0.5] Tag 2
  (:`Pressed`
    (`self.Set Variation` 0 (`self.Tag4`))))

(event `Key|Two`
  (params (Key :type "Key Structure"))
  ;[0.5875 0.1352 1 0.5] Tag 1
  (:`Pressed`
    (`self.Set Variation` 1 (`self.Tag1`))))

(event `Key|Five`
  (params (Key :type "Key Structure"))
  ;[0.5875 0.1352 1 0.5] Tag 2
  (:`Pressed`
    (`self.Set Variation` 1 (`self.Tag4`))))

(event `Key|Three`
  (params (Key :type "Key Structure"))
  ;[0.5875 0.1352 1 0.5] Tag 1
  (:`Pressed`
    (`self.Set Variation` 2 (`self.Tag1`))))

(event `Key|Six`
  (params (Key :type "Key Structure"))
  ;[0.5875 0.1352 1 0.5] Tag 2
  (:`Pressed`
    (`self.Set Variation` 2 (`self.Tag4`))))

(fn `UserConstructionScript`)