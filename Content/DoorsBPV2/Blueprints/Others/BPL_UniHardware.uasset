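; Blueprint function library that maps hardware style enums to static meshes for the DoorsBPV2 doors.
; Each function is a single Select covering handles, entry handles, plates, lock plates, hinges, shutters, sliding-door hardware, rollers or tracks.
; Hinge and shutter lookups return separate door and frame meshes, with some frame meshes shared between styles.
; None and custom options mostly return no mesh, though the custom interior handle returns a default knob.
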(fn `Get Entry Handle Mesh`
  (params (`Handle Style` :type "/Game/DoorsBPV2/Blueprints/Enums/Enum_EntryHandles Enum" :default "NewEnumerator3"))
  (returns (`Handle Mesh` :type "StaticMesh Object Reference"))
  (return (select `/Game/DoorsBPV2/Blueprints/Enums/Enum_EntryHandles` `Handle Style` :`NewEnumerator6` "/Game/DoorsBPV2/Meshes/Hardware/Handles/SM_EntryHandle01_500.SM_EntryHandle01_500" :`NewEnumerator4` "/Game/DoorsBPV2/Meshes/Hardware/Handles/SM_EntryHandle02_500.SM_EntryHandle02_500" :`NewEnumerator5` "/Game/DoorsBPV2/Meshes/Hardware/Handles/SM_EntryHandle02_900.SM_EntryHandle02_900" :`NewEnumerator7` "/Game/DoorsBPV2/Meshes/Hardware/Handles/SM_EntryHandle03_360.SM_EntryHandle03_360" :`NewEnumerator8` "/Game/DoorsBPV2/Meshes/Hardware/Handles/SM_EntryHandle03_800.SM_EntryHandle03_800" :`NewEnumerator9` "/Game/DoorsBPV2/Meshes/Hardware/Handles/SM_EntryHandle04_500.SM_EntryHandle04_500" :`NewEnumerator10` "/Game/DoorsBPV2/Meshes/Hardware/Handles/SM_EntryHandle05_430.SM_EntryHandle05_430" :`NewEnumerator11` "/Game/DoorsBPV2/Meshes/Hardware/Handles/SM_EntryHandle05_780.SM_EntryHandle05_780" :`NewEnumerator12` "/Game/DoorsBPV2/Meshes/Hardware/Handles/SM_EntryHandle06_250.SM_EntryHandle06_250" :`NewEnumerator13` "/Game/DoorsBPV2/Meshes/Hardware/Handles/SM_EntryHandle07_250.SM_EntryHandle07_250" :`NewEnumerator14` "/Game/DoorsBPV2/Meshes/Hardware/Handles/SM_EntryHandle08_200.SM_EntryHandle08_200" :`NewEnumerator15` "/Game/DoorsBPV2/Meshes/Hardware/Handles/SM_EntryHandle09_200.SM_EntryHandle09_200" :!type "StaticMesh Object Reference")))

(fn `Get Handle Mesh`
  (params (`Handle Style` :type "/Game/DoorsBPV2/Blueprints/Enums/Enum_HandleStyle Enum" :default "NewEnumerator7"))
  (returns (`Handle Mesh` :type "StaticMesh Object Reference"))
  (return (select `/Game/DoorsBPV2/Blueprints/Enums/Enum_HandleStyle` `Handle Style` :`NewEnumerator6` "/Game/DoorsBPV2/Meshes/Hardware/Handles/SM_DoorKnob01.SM_DoorKnob01" :`NewEnumerator0` "/Game/DoorsBPV2/Meshes/Hardware/Handles/SM_DoorKnob01.SM_DoorKnob01" :`NewEnumerator1` "/Game/DoorsBPV2/Meshes/Hardware/Handles/SM_DoorKnob01_Button.SM_DoorKnob01_Button" :`NewEnumerator2` "/Game/DoorsBPV2/Meshes/Hardware/Handles/SM_DoorKnob01_Key.SM_DoorKnob01_Key" :`NewEnumerator3` "/Game/DoorsBPV2/Meshes/Hardware/Handles/SM_DoorKnob02.SM_DoorKnob02" :`NewEnumerator4` "/Game/DoorsBPV2/Meshes/Hardware/Handles/SM_Lever_Cont01.SM_Lever_Cont01" :`NewEnumerator11` "/Game/DoorsBPV2/Meshes/Hardware/Handles/SM_Lever_Cont04.SM_Lever_Cont04" :`NewEnumerator8` "/Game/DoorsBPV2/Meshes/Hardware/Handles/SM_Lever_Tempered01.SM_Lever_Tempered01" :`NewEnumerator9` "/Game/DoorsBPV2/Meshes/Hardware/Handles/SM_Lever_Wood01.SM_Lever_Wood01" :`NewEnumerator10` "/Game/DoorsBPV2/Meshes/Hardware/Handles/SM_Lever_Wood02.SM_Lever_Wood02" :`NewEnumerator12` "/Game/DoorsBPV2/Meshes/Hardware/Handles/SM_Lever_Tempered01.SM_Lever_Tempered01" :!type "StaticMesh Object Reference")))

(fn `Get Hinge Meshes`
  (params (`Hinge Style` :type "/Game/DoorsBPV2/Blueprints/Enums/Enum_HingeType Enum" :default "NewEnumerator0"))
  (returns (`Hinge Mesh Door` :type "StaticMesh Object Reference") (`Hinge Mesh Frame` :type "StaticMesh Object Reference"))
  (return (select `/Game/DoorsBPV2/Blueprints/Enums/Enum_HingeType` `Hinge Style` :`NewEnumerator1` "/Game/DoorsBPV2/Meshes/Hardware/Hinges/SM_HingeA_Door.SM_HingeA_Door" :`NewEnumerator3` "/Game/DoorsBPV2/Meshes/Hardware/Hinges/SM_HingeA2_Door.SM_HingeA2_Door" :`NewEnumerator4` "/Game/DoorsBPV2/Meshes/Hardware/Hinges/SM_HingeB_Door.SM_HingeB_Door" :`NewEnumerator5` "/Game/DoorsBPV2/Meshes/Hardware/Hinges/SM_HingeC_Door.SM_HingeC_Door" :`NewEnumerator6` "/Game/DoorsBPV2/Meshes/Hardware/Hinges/SM_HingeD_Door.SM_HingeD_Door" :`NewEnumerator7` "/Game/DoorsBPV2/Meshes/Hardware/Hinges/SM_HingeD2_Door.SM_HingeD2_Door" :`NewEnumerator8` "/Game/DoorsBPV2/Meshes/Hardware/Hinges/SM_HingeD3_Door.SM_HingeD3_Door" :`NewEnumerator9` "/Game/DoorsBPV2/Meshes/Hardware/GlassDoor/SM_Hinge_GlassDoor01.SM_Hinge_GlassDoor01" :!type "StaticMesh Object Reference") (select `/Game/DoorsBPV2/Blueprints/Enums/Enum_HingeType` `Hinge Style` :`NewEnumerator1` "/Game/DoorsBPV2/Meshes/Hardware/Hinges/SM_HingeA_Frame.SM_HingeA_Frame" :`NewEnumerator3` "/Game/DoorsBPV2/Meshes/Hardware/Hinges/SM_HingeA_Frame.SM_HingeA_Frame" :`NewEnumerator4` "/Game/DoorsBPV2/Meshes/Hardware/Hinges/SM_HingeB_Frame.SM_HingeB_Frame" :`NewEnumerator5` "/Game/DoorsBPV2/Meshes/Hardware/Hinges/SM_HingeC_Frame.SM_HingeC_Frame" :`NewEnumerator6` "/Game/DoorsBPV2/Meshes/Hardware/Hinges/SM_HingeD_Frame.SM_HingeD_Frame" :`NewEnumerator7` "/Game/DoorsBPV2/Meshes/Hardware/Hinges/SM_HingeD_Frame.SM_HingeD_Frame" :`NewEnumerator8` "/Game/DoorsBPV2/Meshes/Hardware/Hinges/SM_HingeD_Frame.SM_HingeD_Frame" :`NewEnumerator9` "/Game/DoorsBPV2/Meshes/Hardware/Hinges/SM_HingeA_Frame.SM_HingeA_Frame" :!type "StaticMesh Object Reference")))

(fn `Get Lock Plate Mesh`
  (params (`Lock Plate Style` :type "/Game/DoorsBPV2/Blueprints/Enums/Enum_LockPlates Enum" :default "NewEnumerator0"))
  (returns (`Lock Plate Mesh` :type "StaticMesh Object Reference"))
  (return (select `/Game/DoorsBPV2/Blueprints/Enums/Enum_LockPlates` `Lock Plate Style` :`NewEnumerator1` "/Game/DoorsBPV2/Meshes/Hardware/HPlates/SM_Plate01_Round.SM_Plate01_Round" :`NewEnumerator2` "/Game/DoorsBPV2/Meshes/Hardware/HPlates/SM_Plate04_Round.SM_Plate04_Round" :`NewEnumerator4` "/Game/DoorsBPV2/Meshes/Hardware/HPlates/SM_Plate08_Round.SM_Plate08_Round" :`NewEnumerator5` "/Game/DoorsBPV2/Meshes/Hardware/HPlates/SM_Plate07_Square.SM_Plate07_Square" :!type "StaticMesh Object Reference")))

(fn `Get Plate Mesh`
  (params (`Plate Style` :type "/Game/DoorsBPV2/Blueprints/Enums/Enum_PlateStyles Enum" :default "NewEnumerator5"))
  (returns (`Plate Mesh` :type "StaticMesh Object Reference"))
  (return (select `/Game/DoorsBPV2/Blueprints/Enums/Enum_PlateStyles` `Plate Style` :`NewEnumerator1` "/Game/DoorsBPV2/Meshes/Hardware/HPlates/SM_Plate01_Round.SM_Plate01_Round" :`NewEnumerator3` "/Game/DoorsBPV2/Meshes/Hardware/HPlates/SM_Plate04_Round.SM_Plate04_Round" :`NewEnumerator7` "/Game/DoorsBPV2/Meshes/Hardware/HPlates/SM_Plate08_Round.SM_Plate08_Round" :`NewEnumerator2` "/Game/DoorsBPV2/Meshes/Hardware/HPlates/SM_Plate02_Round.SM_Plate02_Round" :`NewEnumerator6` "/Game/DoorsBPV2/Meshes/Hardware/HPlates/SM_Plate06_Square.SM_Plate06_Square" :`NewEnumerator8` "/Game/DoorsBPV2/Meshes/Hardware/HPlates/SM_LPlate05.SM_LPlate05" :`NewEnumerator9` "/Game/DoorsBPV2/Meshes/Hardware/HPlates/SM_LPlate01.SM_LPlate01" :`NewEnumerator10` "/Game/DoorsBPV2/Meshes/Hardware/HPlates/SM_LPlate02.SM_LPlate02" :`NewEnumerator11` "/Game/DoorsBPV2/Meshes/Hardware/HPlates/SM_LPlate03.SM_LPlate03" :!type "StaticMesh Object Reference")))

(fn `Get Roller Mesh`
  (params (`Roller Style` :type "/Game/DoorsBPV2/Blueprints/Enums/Enum_RollerStyle Enum" :default "NewEnumerator0"))
  (returns (`Roller Mesh` :type "StaticMesh Object Reference"))
  (return (select `/Game/DoorsBPV2/Blueprints/Enums/Enum_RollerStyle` `Roller Style` :`NewEnumerator2` "/Game/DoorsBPV2/Meshes/Hardware/BarnDoor/SM_BarnRoller01.SM_BarnRoller01" :`NewEnumerator3` "/Game/DoorsBPV2/Meshes/Hardware/BarnDoor/SM_BarnRoller02.SM_BarnRoller02" :`NewEnumerator4` "/Game/DoorsBPV2/Meshes/Hardware/BarnDoor/SM_BarnRoller03.SM_BarnRoller03" :`NewEnumerator5` "/Game/DoorsBPV2/Meshes/Hardware/BarnDoor/SM_BarnRoller04.SM_BarnRoller04" :`NewEnumerator6` "/Game/DoorsBPV2/Meshes/Hardware/BarnDoor/SM_BarnRoller05_GlassDoor.SM_BarnRoller05_GlassDoor" :!type "StaticMesh Object Reference")))

(fn `Get Shutter Meshes`
  (params (`Shutter Style` :type "/Game/DoorsBPV2/Blueprints/Enums/Enum_Shutter Enum" :default "NewEnumerator0"))
  (returns (`Shutter Door` :type "StaticMesh Object Reference") (`Shutter Frame` :type "StaticMesh Object Reference"))
  (return (select `/Game/DoorsBPV2/Blueprints/Enums/Enum_Shutter` `Shutter Style` :`NewEnumerator1` "/Game/DoorsBPV2/Meshes/Hardware/Shutter/SM_ShutterA_Door.SM_ShutterA_Door" :`NewEnumerator3` "/Game/DoorsBPV2/Meshes/Hardware/Shutter/SM_ShutterA_Door.SM_ShutterA_Door" :`NewEnumerator4` "/Game/DoorsBPV2/Meshes/Hardware/Shutter/SM_ShutterB_Door.SM_ShutterB_Door" :`NewEnumerator5` "/Game/DoorsBPV2/Meshes/Hardware/GlassDoor/SM_Shutter_GlassDoor01.SM_Shutter_GlassDoor01" :!type "StaticMesh Object Reference") (select `/Game/DoorsBPV2/Blueprints/Enums/Enum_Shutter` `Shutter Style` :`NewEnumerator1` "/Game/DoorsBPV2/Meshes/Hardware/Shutter/SM_ShutterA_Frame.SM_ShutterA_Frame" :`NewEnumerator3` "/Game/DoorsBPV2/Meshes/Hardware/Shutter/SM_ShutterA2_Frame.SM_ShutterA2_Frame" :`NewEnumerator4` "/Game/DoorsBPV2/Meshes/Hardware/Shutter/SM_ShutterB_Frame.SM_ShutterB_Frame" :`NewEnumerator5` "/Game/DoorsBPV2/Meshes/Hardware/Shutter/SM_ShutterA_Frame.SM_ShutterA_Frame" :!type "StaticMesh Object Reference")))

(fn `Get Sliding Handle Mesh`
  (params (`Handle Style` :type "/Game/DoorsBPV2/Blueprints/Enums/Enum_SlidingHandleStyle Enum" :default "NewEnumerator7"))
  (returns (`Handle Mesh` :type "StaticMesh Object Reference"))
  (return (select `/Game/DoorsBPV2/Blueprints/Enums/Enum_SlidingHandleStyle` `Handle Style` :`NewEnumerator0` "/Game/DoorsBPV2/Meshes/Hardware/HandlesSliding/SM_SHandle01.SM_SHandle01" :`NewEnumerator13` "/Game/DoorsBPV2/Meshes/Hardware/HandlesSliding/SM_SHandle02.SM_SHandle02" :`NewEnumerator14` "/Game/DoorsBPV2/Meshes/Hardware/HandlesSliding/SM_SHandle03.SM_SHandle03" :`NewEnumerator15` "/Game/DoorsBPV2/Meshes/Hardware/HandlesSliding/SM_SHandle04.SM_SHandle04" :`NewEnumerator16` "/Game/DoorsBPV2/Meshes/Hardware/HandlesSliding/SM_SHandle05.SM_SHandle05" :`NewEnumerator17` "/Game/DoorsBPV2/Meshes/Hardware/HandlesSliding/SM_SHandle05M.SM_SHandle05M" :!type "StaticMesh Object Reference")))

(fn `Get Sliding Shutter Mesh`
  (params (`Shutter Style` :type "/Game/DoorsBPV2/Blueprints/Enums/Enum_SlidingShutter Enum" :default "NewEnumerator0"))
  (returns (`Shutter Door` :type "StaticMesh Object Reference") (`Shutter Frame` :type "StaticMesh Object Reference"))
  (return (select `/Game/DoorsBPV2/Blueprints/Enums/Enum_SlidingShutter` `Shutter Style` :`NewEnumerator1` "/Game/DoorsBPV2/Meshes/Hardware/Shutter/SM_ShutterS_Door.SM_ShutterS_Door" :!type "StaticMesh Object Reference") (select `/Game/DoorsBPV2/Blueprints/Enums/Enum_SlidingShutter` `Shutter Style` :`NewEnumerator1` "/Game/DoorsBPV2/Meshes/Hardware/Shutter/SM_ShutterS_Frame.SM_ShutterS_Frame" :!type "StaticMesh Object Reference")))

(fn `Get Track Mesh`
  (params (`Track Style` :type "/Game/DoorsBPV2/Blueprints/Enums/Enum_BarnTrackStyle Enum" :default "NewEnumerator0"))
  (returns (`Track Mesh` :type "StaticMesh Object Reference"))
  (return (select `/Game/DoorsBPV2/Blueprints/Enums/Enum_BarnTrackStyle` `Track Style` :`NewEnumerator2` "/Game/DoorsBPV2/Meshes/Hardware/BarnDoor/SM_BarnTrack01.SM_BarnTrack01" :`NewEnumerator3` "/Game/DoorsBPV2/Meshes/Hardware/BarnDoor/SM_BarnTrack02.SM_BarnTrack02" :!type "StaticMesh Object Reference")))