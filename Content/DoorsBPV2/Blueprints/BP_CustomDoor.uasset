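; Configurable door actor built from custom frame, door and hardware meshes, either static or interactive.
; The construction script aligns the door from its mesh bounds, places handles, shutters and instanced hinges and plates, then destroys unused components.
; When movable, player overlap either auto-opens it or shows a text hint for opening through the Interact interface event.
; A timeline swings pivot and handles with sounds, reversing when the player leaves.
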(event `self.ReceiveBeginPlay`
  (bind _handle_inside (`self.Handle Inside`))
  ;[1 1 1] initially open door - hide text hint
  (`self.TextMarkerVisibility` false)
  (if (`self.InitiallyOpen`)
    ;[1 1 1] open close door
    (set `self.DoorIsOpen` true :!label _label)
    (bind (_direction _opendoor _handles) (`Timeline|Timeline_0` :!label _label_2)
      (:`Update`
        (if (`self.isMovable`)
          (`SceneComponent.K2_SetRelativeRotation` (`self.Pivot1`) (`KismetMathLibrary.MakeRotator` 0.0 0.0 (`KismetMathLibrary.Lerp` 0.0 (`self.DesiredOpeningRotation`) _opendoor)) false false)
          (if (`self.AddHandleInside`)
            (if (or (`self.MoveHandleOutside`) (not (`KismetSystemLibrary.IsValid` (`self.HandleMeshOutside`))))
              (bind _returnvalue (`KismetMathLibrary.MakeRotator` (`KismetMathLibrary.Lerp` 0.0 (`self.DesiredHandleRotation`) _handles)))
              (`SceneComponent.K2_SetRelativeRotation` _handle_inside _returnvalue false false)
              (`SceneComponent.K2_SetRelativeRotation` (`self.Handle Outside`) _returnvalue false false)
              (else
                (`SceneComponent.K2_SetRelativeRotation` _handle_inside _returnvalue false false))))))
      (:`Opening sound`
        ;[1 1 1] Sound
        (`/Engine/EditorBlueprintResources/StandardMacros.FlipFlop`
          (:`A`
            (`GameplayStatics.PlaySoundAtLocation` (`self.OpeningSound`) (0.0 0.0 0.0) (struct) 1.0 1.0 0.0 null null null null))))
      (:`ClosingSound`
        (`/Engine/EditorBlueprintResources/StandardMacros.FlipFlop`
          (:`B`
            (`GameplayStatics.PlaySoundAtLocation` (`self.ClosingSound`) (0.0 0.0 0.0) (struct) 1.0 1.0 0.0 null null null null)))))))

(event `OpenDoor`
  ;[1 1 1] open close door
  (if (`self.InRange`)
    (`self.TextMarkerVisibility` false)
    (goto _label)))

(event `self.ReceiveActorBeginOverlap`
  (params (OtherActor :type "Actor Object Reference"))
  ;[1 1 1] open close door
  (set `self.InRange` true)
  (if (`self.InitiallyOpen`)
    (set `self.InitiallyOpen` false)
    (elif (and (`self.isMovable`) (== OtherActor (`GameplayStatics.GetPlayerPawn` 0)))
      (if (`self.AutoOpen`)
        (goto _label)
        (else
          (`self.TextMarkerVisibility` (`self.InRange`) :!label _label_3)
          (if (`self.DoorIsOpen`)
            (set `self.DoorIsOpen` false)
            (goto _label_2 :!via `Reverse`)))))))

(event `self.ReceiveActorEndOverlap`
  (params (OtherActor :type "Actor Object Reference"))
  ;[1 1 1] open close door
  (set `self.InRange` false)
  (if (and (`self.isMovable`) (== OtherActor (`GameplayStatics.GetPlayerPawn` 0)))
    (if (`self.AutoOpen`)
      (goto _label_2 :!via `Reverse`)
      (else
        (goto _label_3)))))

(event `/Game/DoorsBPV2/Blueprints/Others/BPI_Doors_Interaction.Interact`
  ;[1 0.7839 0.2481] Blueprint Interface Actions
  (`self.OpenDoor`))

(fn `AddHardwareOffset`
  (bind (_handle_height _lockheight) (`self.GetHandleHeight`))
  (bind _handlehorizontaloffset (`self.HandleHorizontalOffset`))
  (bind (_scaled_door_size_x _scaled_door_size_y) (`KismetMathLibrary.BreakVector` (`self.Scaled Door Size`)))
  (`|ExecutionSequence`
    (:`then_0`
      (`SceneComponent.K2_AddLocalOffset` (`self.ShutterDoor`) (`KismetMathLibrary.MakeVector` 0.0 0.0 _handle_height) false false)
      (`SceneComponent.K2_AddLocalOffset` (`self.ShutterDoor`) (`self.Door Offset Handle`) false false)
      (`SceneComponent.K2_AddLocalOffset` (`self.ShutterFrame`) (`self.Door Offset Handle`) false false))
    (:`then_1`
      (`SceneComponent.K2_AddLocalOffset` (`self.ShutterFrame`) (`KismetMathLibrary.MakeVector` -2.0 (+ _scaled_door_size_y 0.4) _handle_height) false false))
    (:`then_2`
      (`SceneComponent.K2_AddLocalOffset` (`self.Handle Inside`) (`KismetMathLibrary.MakeVector` (`self.HandleOffset`) _handlehorizontaloffset _handle_height) false false)
      (`SceneComponent.K2_AddLocalOffset` (`self.Handle Outside`) (`KismetMathLibrary.MakeVector` (* (+ (`self.HandleOffset`) (`self.Door Thickness Offset`) (select `bool` (`self.AddHandlePlateOutside`) :`false` (`self.HandleOffsetOutside`))) -1.0) (`self.HandleHorizontalOffset`) (+ (`self.HandleVerticalOffsetOutside`) (`self.GetHandleHeight`))) false false))
    (:`then_3`
      (`SceneComponent.K2_AddLocalOffset` (`self.HandlePlates`) (`KismetMathLibrary.MakeVector` 0.0 _handlehorizontaloffset _handle_height) false false))
    (:`then_4`
      (`SceneComponent.K2_AddLocalOffset` (`self.LockPlates`) (`KismetMathLibrary.MakeVector` 0.0 _handlehorizontaloffset (+ _handle_height _lockheight)) false false))
    (:`then_5`
      (`SceneComponent.K2_AddLocalOffset` (`self.HingesFrame`) (0.2 -0.5 0.0) false false))))

(fn `AddHingesInstances`
  (bind _hingesdoor (`self.HingesDoor`))
  (bind _materialshardware (`self.MaterialsHardware`))
  (bind _hingesframe (`self.HingesFrame`))
  (`KismetArrayLibrary.Array_Clear` (`self.TransformsHW`))
  (`|ExecutionSequence`
    (:`then_0`
      (`StaticMeshComponent.SetStaticMesh` _hingesframe (`self.HingesFrameMesh`))
      (`self.Set Material IDs` _hingesframe _materialshardware)
      (bind _transforms (`self.GetHingesTransforms` true))
      (`InstancedStaticMeshComponent.AddInstances` _hingesframe _transforms false false true))
    (:`then_1`
      (`StaticMeshComponent.SetStaticMesh` _hingesdoor (`self.HingesDoorMesh`))
      (`self.Set Material IDs` _hingesdoor _materialshardware)
      (bind _transforms_2 (`self.GetHingesTransforms` false))
      (`InstancedStaticMeshComponent.AddInstances` _hingesdoor _transforms_2 false false true))))

(fn `AddPlateInstances`
  (bind _transforms (`self.Make Transforms in Out`))
  (bind _handleplates (`self.HandlePlates`))
  (bind _lockplates (`self.LockPlates`))
  (bind _materialshandles (`self.MaterialsHandles`))
  (`|ExecutionSequence`
    (:`then_0`
      ;[0.571 0.7923 1] Door 1
      (`self.Set Mesh And Materials` _handleplates (`self.PlateMesh`) _materialshandles)
      (`InstancedStaticMeshComponent.AddInstances` _handleplates (select `bool` (`self.AddHandlePlateOutside`) :`false` (`self.Plate TransformInside`) :`true` _transforms) false false true))
    (:`then_1`
      (`self.Set Mesh And Materials` _lockplates (`self.LockPlateMesh`) _materialshandles)
      (`InstancedStaticMeshComponent.AddInstances` _lockplates _transforms false false true))))

(fn `CalculateDoorSize`
  (returns (`Door Size` :type "Vector Structure") (`Scaled Size` :type "Vector Structure"))
  (bind _door_rotation_correction (`self.Door Rotation Correction`))
  (bind _door_rotation_correction_2 (`self.Door Rotation Correction`))
  (bind _returnvalue (* (.y (`.BoxExtent` (`KismetMathLibrary.BreakBoxSphereBounds` (`StaticMesh.GetBounds` (`self.GetDoor` 0))))) 2.0))
  (bind _returnvalue_2 (* (.x (`.BoxExtent` (`KismetMathLibrary.BreakBoxSphereBounds` (`StaticMesh.GetBounds` (`self.GetDoor` 0))))) 2.0))
  (bind _returnvalue_3 (* (.z (`.BoxExtent` (`KismetMathLibrary.BreakBoxSphereBounds` (`StaticMesh.GetBounds` (`self.GetDoor` 0))))) 2.0))
  (bind _returnvalue_4 (* _returnvalue_2 (.x (`self.Custom Door Scale`))))
  (bind _returnvalue_5 (* _returnvalue (.y (`self.Custom Door Scale`))))
  (return (`KismetMathLibrary.MakeVector` (select `/Game/DoorsBPV2/Blueprints/Enums/Enum_Rotation` _door_rotation_correction_2 :`NewEnumerator0` _returnvalue_2 :`NewEnumerator1` _returnvalue :`NewEnumerator2` _returnvalue_2 :`NewEnumerator3` _returnvalue) (select `/Game/DoorsBPV2/Blueprints/Enums/Enum_Rotation` _door_rotation_correction_2 :`NewEnumerator0` _returnvalue :`NewEnumerator1` _returnvalue_2 :`NewEnumerator2` _returnvalue :`NewEnumerator3` _returnvalue_2) _returnvalue_3) (`KismetMathLibrary.MakeVector` (select `/Game/DoorsBPV2/Blueprints/Enums/Enum_Rotation` _door_rotation_correction :`NewEnumerator0` _returnvalue_4 :`NewEnumerator1` _returnvalue_5 :`NewEnumerator2` _returnvalue_4 :`NewEnumerator3` _returnvalue_5) (select `/Game/DoorsBPV2/Blueprints/Enums/Enum_Rotation` _door_rotation_correction :`NewEnumerator0` _returnvalue_5 :`NewEnumerator1` _returnvalue_4 :`NewEnumerator2` _returnvalue_5 :`NewEnumerator3` _returnvalue_4) (* _returnvalue_3 (.z (`self.Custom Door Scale`))))))

(fn `Change Variation Material`
  (params (Part :type "/Game/DoorsBPV2/Blueprints/Enums/Enum_DoorParts Enum" :default "NewEnumerator0") (Materials :type "Array of MaterialInterface Object Reference"))
  (for _array_element (select `/Game/DoorsBPV2/Blueprints/Enums/Enum_DoorParts` Part :`NewEnumerator0` (`self.DoorComponents`) :`NewEnumerator1` (`|MakeArray` (`self.Frame`)))
    (`/Engine/EditorBlueprintResources/StandardMacros.IsValid` _array_element
      (:`Is Valid`
        (`self.Set Material IDs` _array_element Materials)))))

(fn `Change Variation Meshes`
  (params (InputPin :type "/Game/DoorsBPV2/Blueprints/Enums/Enum_DoorParts Enum" :default "NewEnumerator0") (InputPin1 :type "StaticMesh Object Reference"))
  (for _array_element (select `/Game/DoorsBPV2/Blueprints/Enums/Enum_DoorParts` InputPin :`NewEnumerator0` (`self.DoorComponents`) :`NewEnumerator1` (`|MakeArray` (`self.Frame`)))
    (`/Engine/EditorBlueprintResources/StandardMacros.IsValid` _array_element
      (:`Is Valid`
        (`SceneComponent.SetMobility` _array_element "Movable")
        (`StaticMeshComponent.SetStaticMesh` _array_element InputPin1)))))

(fn `Get Door Size`
  (returns (`Thickness X` :type "Float (double-precision)") (`Width Y` :type "Float (double-precision)") (`Height Z` :type "Float (double-precision)"))
  (return (.x (`self.Custom  Door Size`)) (.y (`self.Custom  Door Size`)) (.z (`self.Custom  Door Size`))))

(fn `Get Valid Material`
  (params (Default :type "MaterialInterface Object Reference") (Optional :type "MaterialInterface Object Reference"))
  (returns (Valid :type "MaterialInterface Object Reference"))
  (return (select `bool` (`KismetSystemLibrary.IsValid` Optional) :`false` Default :`true` Optional)))

(fn `Get Valid Materials`
  (params (Default :type "Array of MaterialInterface Object Reference") (Optional :type "Array of MaterialInterface Object Reference"))
  (returns (Valid :type "Array of MaterialInterface Object Reference"))
  (return (select `bool` (`KismetArrayLibrary.Array_IsValidIndex` Optional) :`false` Default :`true` Optional)))

(fn `GetDoor`
  (params (`Mesh ID` :type Integer))
  (returns (`Static Mesh` :type "StaticMesh Object Reference") (Materials :type "Array of MaterialInterface Object Reference"))
  (bind (_staticmesh _materials) (break `/Game/DoorsBPV2/Blueprints/Structs/BPS_MeshAndMaterials` (`|GetArrayItem` (`self.DoorMeshes`) `Mesh ID`)))
  (return _staticmesh _materials))

(fn `GetHandleHeight`
  (returns (`Handle Height` :type "Float (double-precision)") (LockHeight :type "Float (double-precision)"))
  (return (/ (`self.HandleHeight`) 1.0) (/ (`self.LockHeight`) 1.0)))

(fn `GetHingesTransforms`
  (params (Frame :type Boolean))
  (returns (Transforms :type "Array of Transform Structure"))
  (bind (_scaled_door_size_x _scaled_door_size_y _scaled_door_size_z) (`KismetMathLibrary.BreakVector` (`self.Scaled Door Size`)))
  (`KismetArrayLibrary.Array_Clear` (`self.TransformsHW`))
  (for _index (range (`self.HingesAmount`))
    (`KismetArrayLibrary.Array_Add` (`self.TransformsHW`) (`KismetMathLibrary.MakeTransform` (`KismetMathLibrary.MakeVector` 0.0 0.0 (+ (`self.EdgeDistance`) (* _index (/ (- _scaled_door_size_z (* (`self.EdgeDistance`) 2.0)) (- (`self.HingesAmount`) 1))))))))
  (return (`self.TransformsHW`)))

(fn `isMovable`
  (returns (isMovable :type Boolean))
  (return (`|EnumEquality` (`self.DoorMobility`) "Movable")))

(fn `Make Transforms in Out`
  (returns (Transforms :type "Array of Transform Structure"))
  (return (`|MakeArray` (`|GetArrayItem` (`self.Plate TransformInside`)) (`KismetMathLibrary.MakeTransform` (`KismetMathLibrary.MakeVector` (- -4.0 (`self.Door Thickness Offset`))) (struct) (-1.0 -1.0 1.0)))))

(fn `Movable Door Settings`
  (`|ExecutionSequence`
    (:`then_0`
      ;[1 1 1] Movable Door Settings
      (if (`self.isMovable`)
        (`SceneComponent.SetRelativeScale3D` (`self.CollisionBox`) (`self.CollisionScale`))
        (`SceneComponent.K2_AddRelativeLocation` (`self.CollisionBox`) (`self.CollisionLocationOffset`) false false)
        (`self.TextMarkerSettings`)))
    (:`then_1`
      ;[1 1 1] set text hint visibility
      (if (not (and (`self.isMovable`) (not (`self.AutoOpen`))))
        (`self.TextMarkerVisibility` false)))))

(fn `Pre Align Door`
  (bind _attachdoor (`self.AttachDoor`))
  (`|ExecutionSequence`
    (:`then_0`
      (bind _offset (`/Game/DoorsBPV2/Blueprints/Others/BPL_UniDoors.GetCustomOffset` (`self.GetDoor` 0) (`self.Door Rotation Correction`) (`self.Custom Door Scale`)))
      (set `self.Calculated Door Offset` _offset))
    (:`then_1`
      (`SceneComponent.K2_AddLocalRotation` (`self.AttachDoor`) (`KismetMathLibrary.MakeRotator` 0.0 0.0 (select `/Game/DoorsBPV2/Blueprints/Enums/Enum_Rotation` (`self.Door Rotation Correction`) :`NewEnumerator1` 90.0 :`NewEnumerator2` 180.0 :`NewEnumerator3` 270.0 :!type "Float (single-precision)")) false false)
      (`SceneComponent.K2_AddLocalOffset` _attachdoor (+ (`self.Calculated Door Offset`) (`self.Door Offset Hinge`)) false false)
      (`SceneComponent.SetRelativeScale3D` _attachdoor (`self.Custom Door Scale`)))))

(fn `Remove Obsolete Meshes`
  (`|ExecutionSequence`
    (:`then_0`
      ;[0.571 0.7923 1] remove obsolete meshes
      (`|ExecutionSequence`
        (:`then_0`
          (if (not (`self.isMovable`))
            (`ActorComponent.K2_DestroyComponent` (`self.CollisionBox`))))
        (:`then_2`
          (if (not (`self.AddHandlePlateInside`))
            (`ActorComponent.K2_DestroyComponent` (`self.HandlePlates`))))
        (:`then_3`
          (if (not (`self.AddLockPlates`))
            (`ActorComponent.K2_DestroyComponent` (`self.LockPlates`))))
        (:`then_4`
          (if (not (`self.AddHandleInside`))
            (`ActorComponent.K2_DestroyComponent` (`self.Handle Inside`))))
        (:`then_5`
          (if (not (`self.AddHandleOutside`))
            (`ActorComponent.K2_DestroyComponent` (`self.Handle Outside`))))
        (:`then_6`
          (if (not (`self.AddHinges`))
            (`ActorComponent.K2_DestroyComponent` (`self.HingesFrame`))
            (`ActorComponent.K2_DestroyComponent` (`self.HingesDoor`))))
        (:`then_7`
          (if (not (`self.AddShutter`))
            (`ActorComponent.K2_DestroyComponent` (`self.ShutterFrame`))
            (`ActorComponent.K2_DestroyComponent` (`self.ShutterDoor`))))))))

(fn `Set Material IDs`
  (params (Mesh :type "StaticMeshComponent Object Reference") (Materials :type "Array of MaterialInterface Object Reference"))
  (for (_array_element _array_index) Materials
    (`/Engine/EditorBlueprintResources/StandardMacros.IsValid` _array_element
      (:`Is Valid`
        (`/Engine/EditorBlueprintResources/StandardMacros.IsValid` (`PrimitiveComponent.GetMaterial` Mesh _array_index)
          (:`Is Valid`
            (`PrimitiveComponent.SetMaterial` Mesh _array_index _array_element)))))))

(fn `Set Mesh And Materials`
  (params (Component :type "StaticMeshComponent Object Reference") (NewMesh :type "StaticMesh Object Reference") (Materials :type "Array of MaterialInterface Object Reference (by ref)"))
  (`StaticMeshComponent.SetStaticMesh` Component NewMesh)
  (`self.Set Material IDs` Component Materials))

(fn `SetHardwareMeshes`
  (bind _materialshardware (`self.MaterialsHardware`))
  (`|ExecutionSequence`
    (:`then_0`
      (`self.Set Mesh And Materials` (`self.Handle Inside`) (`self.HandleMesh`) (`self.MaterialsHandles`)))
    (:`then_1`
      (`self.Set Mesh And Materials` (`self.Handle Outside`) (select `bool` (`KismetSystemLibrary.IsValid` (`self.HandleMeshOutside`)) :`false` (`self.HandleMesh`) :`true` (`self.HandleMeshOutside`)) (`self.MaterialsHandles`)))
    (:`then_2`
      (`self.Set Mesh And Materials` (`self.ShutterDoor`) (select `bool` (`KismetSystemLibrary.IsValid` (`self.ShutterDoorMesh`)) :`false` "/Game/DoorsBPV2/Meshes/Hardware/Shutter/SM_ShutterA_Door.SM_ShutterA_Door" :`true` (`self.ShutterDoorMesh`)) _materialshardware))
    (:`then_3`
      (`self.Set Mesh And Materials` (`self.ShutterFrame`) (select `bool` (`KismetSystemLibrary.IsValid` (`self.ShutterFrameMesh`)) :`false` "/Game/DoorsBPV2/Meshes/Hardware/Shutter/SM_ShutterA_Frame.SM_ShutterA_Frame" :`true` (`self.ShutterFrameMesh`)) _materialshardware))))

(fn `Setup Door`
  (bind (_door_offset_handle_x _door_offset_handle_y _door_offset_handle_z) (`KismetMathLibrary.BreakVector` (`self.Door Offset Handle`)))
  (bind (_door_offset_frame_x _door_offset_frame_y _door_offset_frame_z) (`KismetMathLibrary.BreakVector` (`self.Door Offset Frame`)))
  (bind (_scaled_door_size_x _scaled_door_size_y) (`KismetMathLibrary.BreakVector` (`self.Scaled Door Size`)))
  (`|ExecutionSequence`
    (:`then_0`
      ;[0.571 0.7923 1] Door Mesh
      (`SceneComponent.SetMobility` (`self.Pivot1`) (`self.DoorMobility`))
      (bind (_door_size _scaled_size) (`self.CalculateDoorSize`))
      (bind _output_get (set `self.Custom  Door Size` _door_size))
      (set `self.Scaled Door Size` _scaled_size)
      (`SceneComponent.K2_SetRelativeLocation` (`self.Pivot1`) (`KismetMathLibrary.MakeVector` (+ _door_offset_frame_x 0.5) (+ _door_offset_frame_y -0.2 (* (.y _output_get) -0.5)) (+ _door_offset_frame_z 1.0)) false false)
      (`SceneComponent.K2_SetRelativeLocation` (`self.HingesFrame`) (`KismetMathLibrary.MakeVector` (+ _door_offset_frame_x 0.5) (+ _door_offset_frame_y -0.2 (* (.y _output_get) -0.5)) (+ _door_offset_frame_z 1.0)) false false)
      (`SceneComponent.K2_SetRelativeLocation` (`self.ShutterFrame`) (`KismetMathLibrary.MakeVector` (+ _door_offset_frame_x 0.5) (+ _door_offset_frame_y -0.2 (* (.y _output_get) -0.5)) (+ _door_offset_frame_z 1.0)) false false)
      (`SceneComponent.K2_SetRelativeLocation` (`self.AttachHandle`) (`KismetMathLibrary.MakeVector` (+ _door_offset_handle_x -0.5) (+ _door_offset_handle_y _scaled_door_size_y) _door_offset_handle_z) false false))
    (:`then_1`
      (for _array_element (`self.DoorMeshes`)
        (bind _returnvalue (`AddComponent|NODE_AddStaticMeshComponent-5`))
        (`KismetArrayLibrary.Array_Add` (`self.DoorComponents`) _returnvalue)
        (bind (_staticmesh _materials) (break `/Game/DoorsBPV2/Blueprints/Structs/BPS_MeshAndMaterials` _array_element))
        (`self.Set Mesh And Materials` _returnvalue _staticmesh _materials)
        (`SceneComponent.K2_AttachToComponent` _returnvalue (`self.AttachDoor`) "None" "KeepRelative" "KeepRelative" "KeepRelative" true)))
    (:`then_2`
      (`SceneComponent.K2_AddRelativeRotation` (`self.Pivot1`) (`KismetMathLibrary.MakeRotator` 0.0 0.0 (* (`self.DoorRotation`) -1.0)) false false))))

(fn `Setup Frame`
  (bind _frame (`self.Frame`))
  (`|ExecutionSequence`
    (:`then_0`
      ;[0.571 0.7923 1] Frame Mesh
      (`self.Set Mesh And Materials` (`self.Frame`) (`self.CustomFrameMesh`) (`self.MaterialsFrame`))
      (`SceneComponent.SetRelativeScale3D` (`self.AttachFrame`) (`KismetMathLibrary.MakeVector` 1.0 (select `bool` (`self.Flip Door`) :`false` 1.0 :`true` -1.0) 1.0)))
    (:`then_1`
      (`SceneComponent.SetRelativeScale3D` _frame (`self.Frame Scale`))
      (`SceneComponent.K2_AddRelativeRotation` _frame (`KismetMathLibrary.MakeRotator` 0.0 0.0 (select `/Game/DoorsBPV2/Blueprints/Enums/Enum_Rotation` (`self.Frame Rotation Correction`) :`NewEnumerator1` 90.0 :`NewEnumerator2` 180.0 :`NewEnumerator3` 270.0)) false false))))

(fn `TextMarkerSettings`
  (bind _textrender (`self.TextRender`))
  (`TextRenderComponent.K2_SetText` _textrender (`self.TextHint`))
  (`TextRenderComponent.K2_SetText` (`self.TextRender1`) (`self.TextHint`))
  (`TextRenderComponent.SetTextRenderColor` _textrender (`self.TextRenderColor`))
  (`TextRenderComponent.SetTextRenderColor` (`self.TextRender1`) (`self.TextRenderColor`))
  (`SceneComponent.K2_AddLocalOffset` _textrender (`self.TextOffsetOut`) false false)
  (`SceneComponent.K2_AddLocalOffset` (`self.TextRender1`) (`self.TextOffsetIn`) false false))

(fn `TextMarkerVisibility`
  (params (Visibility :type Boolean))
  (`SceneComponent.SetVisibility` (`self.TextRender1`) Visibility false)
  (`SceneComponent.SetVisibility` (`self.TextRender`) Visibility false))

(fn `UserConstructionScript`
  (locals (NewLocalVar_0 :type "Rotator Structure" :default (struct)) (NewLocalVar_1 :type "Array of Transform Structure"))
  (`|ExecutionSequence`
    (:`then_0`
      (`self.Setup Frame`)
      (`self.Setup Door`)
      (`self.Pre Align Door`))
    (:`then_1`
      (`self.SetHardwareMeshes`)
      (`self.AddHingesInstances`)
      (`self.AddPlateInstances`)
      (`self.AddHardwareOffset`))
    (:`then_2`
      (`self.Movable Door Settings`)
      (`self.Remove Obsolete Meshes`))))